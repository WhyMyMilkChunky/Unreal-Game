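; RTS-style player controller that drives the camera pawn and handles unit selection and move orders.
; Screen-edge, Enhanced Input and middle-mouse input set direction, rotation and zoom values, which MoveCamera applies each tick with speed scaled by spring arm length.
; Left click signals the HUD to start or stop selection and clears units on a missed trace.
; Right click builds a square-root-sized grid at the cursor and writes each unit's Blackboard TargetLocation.
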(event Input|EnhancedActionEvents|EnhancedInputActionAC_Rotate
  (params (ActionValue :type Vector%202D%20Structure) (ElapsedSeconds :type Float%20%28double-precision%29) (TriggeredSeconds :type Float%20%28double-precision%29) (InputAction :type Input%20Action%20Object%20Reference :default "/Game/Controls/Input/AC_Rotate.AC_Rotate"))
  ;[0.4662 0.8486 1] Gamepad Rotate
  (:Triggered
    (if (> (.x ActionValue) 0.4)
      (Camera|RotateCameraController (.x ActionValue) :!label _label)
      (elif (< (.x ActionValue) -0.4)
        (goto _label)
        (else
          (Camera|ResetRotationController :!label _label_2)))))
  (:Completed
    (goto _label_2)))

(event Input|EnhancedActionEvents|EnhancedInputActionAC_Move
  (params (ActionValue :type Vector%202D%20Structure) (ElapsedSeconds :type Float%20%28double-precision%29) (TriggeredSeconds :type Float%20%28double-precision%29) (InputAction :type Input%20Action%20Object%20Reference :default "/Game/Controls/Input/AC_Move.AC_Move"))
  (bind (_x _y) (Math|Vector2D|BreakVector2D ActionValue))
  ;[1 0.8439 0.2628] Regular Move Dir
  (:Triggered
    (bind _output_get (Variables|Movement|SetMoveDir (Math|Vector|MakeVector _x _y 0.0)))
    (Variables|Movement|SetKeyDirX (.x _output_get))
    (Variables|Movement|SetKeyDirY (.y _output_get)))
  (:Completed
    (bind _output_get_2 (Variables|Movement|SetMoveDir (Math|Vector|MakeVector _x _y 0.0)))
    (Variables|Movement|SetKeyDirY (.y _output_get_2))
    (Variables|Movement|SetKeyDirX (.x _output_get_2))))

(event Input|EnhancedActionEvents|EnhancedInputActionZoom
  (params (ActionValue :type Vector%202D%20Structure) (ElapsedSeconds :type Float%20%28double-precision%29) (TriggeredSeconds :type Float%20%28double-precision%29) (InputAction :type Input%20Action%20Object%20Reference :default "/Game/Controls/Input/Zoom.Zoom"))
  (bind _x (Math|Vector2D|BreakVector2D ActionValue))
  ;[0.4633 1 0.3313] Zoom
  (:Triggered
    (if (< _x 0.0)
      (Variables|View|SetCameraZoom (+ (Variables|View|GetCameraZoom) 1e+02))
      (else
        (if (> _x 0.0) :!label _label
          (Variables|View|SetCameraZoom (- (Variables|View|GetCameraZoom) 1e+02))
          (else
            (Variables|View|SetCameraZoom 0.0))))))
  (:Completed
    (goto _label)))

(event Input|EnhancedActionEvents|EnhancedInputActionAC_ControllerZoom
  (params (ActionValue :type Vector%202D%20Structure) (ElapsedSeconds :type Float%20%28double-precision%29) (TriggeredSeconds :type Float%20%28double-precision%29) (InputAction :type Input%20Action%20Object%20Reference :default "/Game/Controls/Input/AC_ControllerZoom.AC_ControllerZoom"))
  ;[0.4633 1 0.3313] Zoom
  (if (> (.x ActionValue) 0.4)
    (Variables|View|SetCameraZoom (- (Variables|View|GetCameraZoom) 1.0))
    (elif (< (.x ActionValue) -0.4)
      (Variables|View|SetCameraZoom (+ (Variables|View|GetCameraZoom) 1.0))
      (elif (< (.X (Math|Vector2D|BreakVector2D (stale Input|EnhancedActionEvents|EnhancedInputActionZoom ActionValue))) 0.0)
        (Variables|View|SetCameraZoom (+ (Variables|View|GetCameraZoom) 1e+02))
        (elif (> (.X (Math|Vector2D|BreakVector2D (stale Input|EnhancedActionEvents|EnhancedInputActionZoom ActionValue))) 0.0)
          (Variables|View|SetCameraZoom (- (Variables|View|GetCameraZoom) 1e+02))
          (else
            (Variables|View|SetCameraZoom 0.0)))))))

(event EventBeginPlay
  (CallFunction|GetInputs (PlayerController|LocalPlayerSubsystems|GetEnhancedInputLocalPlayerSubsystem))
  (bind _returnvalue (Actor|GetActorOfClass "/Game/Blueprints/Resources/BP_ResourceManager.BP_ResourceManager_C"))
  (Variables|Default|Setresourcemanager _returnvalue))

(event EventTick
  (params (DeltaSeconds :type Float%20%28single-precision%29))
  (Camera|MoveCamera))

(event Input|MouseEvents|MouseX
  (params (AxisValue :type Float%20%28single-precision%29))
  (bind _returnvalue (Viewport|GetViewportSize))
  (bind _returnvalue_2 (Game|GetPlayerController 0))
  (bind (_locationx _locationy) (Game|Player|GetMousePosition _returnvalue_2))
  (bind _locationx_2 (Game|Player|GetMousePosition _returnvalue_2))
  (bind _returnvalue_3 (/ _locationy (.y _returnvalue)))
  (bind _returnvalue_4 (/ _locationx (.x _returnvalue)))
  ;[1 0.8959 0.1604] Move Edge Scrolling
  (if (>= _returnvalue_4 0.975)
    (bind _output_get (Variables|Movement|SetEdgeDirX 1.0))
    (Variables|Movement|SetMoveDir (Math|Vector|MakeVector (.x (Variables|Movement|GetMoveDir)) _output_get (.z (Variables|Movement|GetMoveDir))))
    (elif (<= _returnvalue_4 0.025)
      (bind _output_get_2 (Variables|Movement|SetEdgeDirX -1.0))
      (Variables|Movement|SetMoveDir (Math|Vector|MakeVector (.x (Variables|Movement|GetMoveDir)) _output_get_2 (.z (Variables|Movement|GetMoveDir))))
      (elif (>= _returnvalue_3 0.975)
        (bind _output_get_3 (Variables|Movement|SetEdgeDirY -1.0))
        (Variables|Movement|SetMoveDir (Math|Vector|MakeVector _output_get_3 (.y (Variables|Movement|GetMoveDir)) (.z (Variables|Movement|GetMoveDir))))
        (elif (<= _returnvalue_3 0.025)
          (bind _output_get_4 (Variables|Movement|SetEdgeDirY 1.0))
          (Variables|Movement|SetMoveDir (Math|Vector|MakeVector _output_get_4 0.0 (.z (Variables|Movement|GetMoveDir))))
          (else
            (Variables|Movement|SetMoveDir (Math|Vector|MakeVector (Variables|Movement|GetKeyDirX) (Variables|Movement|GetKeyDirY) 0.0))
            ;[0.06772 0.3853 1] Rotate
            (if (stale Input|MouseEvents|MiddleMouseButton _output_get)
              (Variables|View|SetRotSpeed (- (Variables|View|GetMouseRotPos) (.LocationX (Game|Player|GetMousePosition))))
              (if (> _locationx_2 (stale Input|MouseEvents|MiddleMouseButton _output_get_2))
                (Variables|View|SetRotAxis 1.0)
                (elif (< _locationx_2 (stale Input|MouseEvents|MiddleMouseButton _output_get_2))
                  (Variables|View|SetRotAxis -1.0))))))))))

(event Input|MouseEvents|MouseY
  (params (AxisValue :type Float%20%28single-precision%29))
  (bind _returnvalue (Viewport|GetViewportSize))
  (bind _returnvalue_2 (Game|GetPlayerController 0))
  (bind (_locationx _locationy) (Game|Player|GetMousePosition _returnvalue_2))
  (bind _locationx_2 (Game|Player|GetMousePosition _returnvalue_2))
  (bind _returnvalue_3 (/ _locationy (.y _returnvalue)))
  ;[1 0.8959 0.1604] Move Edge Scrolling
  (if (>= _returnvalue_3 0.975)
    (bind _output_get (Variables|Movement|SetEdgeDirY -1.0))
    (Variables|Movement|SetMoveDir (Math|Vector|MakeVector _output_get (.y (Variables|Movement|GetMoveDir)) (.z (Variables|Movement|GetMoveDir))))
    (elif (<= _returnvalue_3 0.025)
      (bind _output_get_2 (Variables|Movement|SetEdgeDirY 1.0))
      (Variables|Movement|SetMoveDir (Math|Vector|MakeVector _output_get_2 0.0 (.z (Variables|Movement|GetMoveDir))))
      (else
        (Variables|Movement|SetMoveDir (Math|Vector|MakeVector (Variables|Movement|GetKeyDirX) (Variables|Movement|GetKeyDirY) 0.0))
        ;[0.06772 0.3853 1] Rotate
        (if (stale Input|MouseEvents|MiddleMouseButton _output_get)
          (Variables|View|SetRotSpeed (- (Variables|View|GetMouseRotPos) (.LocationX (Game|Player|GetMousePosition))))
          (if (> _locationx_2 (stale Input|MouseEvents|MiddleMouseButton _output_get_2))
            (Variables|View|SetRotAxis 1.0)
            (elif (< _locationx_2 (stale Input|MouseEvents|MiddleMouseButton _output_get_2))
              (Variables|View|SetRotAxis -1.0))))))))

(event Input|KeyboardEvents|DebugKeyH
  (params (Key :type Key%20Structure :default "None") (ActionValue :type Input%20Action%20Value%20Structure))
  (:Released
    (Default|ResourcesTest (Variables|Default|Getresourcemanager))))

(event Input|MouseEvents|LeftMouseButton
  (params (Key :type Key%20Structure :default "None"))
  (bind _returnvalue (HUD|GetHUD))
  ;[1 0 0.8618] Selection
  (:Pressed
    (Class|SelectionInterface|StartSelection(Message) _returnvalue)
    (if (not (.ReturnValue (Game|Player|GetHitResultUnderCursorbyChannel "TraceTypeQuery3" true)))
      (Selecting|ClearUnitSelection)))
  (:Released
    (Class|SelectionInterface|StopSelection(Message) _returnvalue)))

(event Input|GamepadEvents|GamepadFaceButtonBottom
  (params (Key :type Key%20Structure :default "None"))
  (bind _returnvalue (Viewport|GetViewportSize))
  (bind _returnvalue_2 (* (.y _returnvalue) 0.5))
  (bind _returnvalue_3 (* (.x _returnvalue) 0.5))
  (bind (_worldlocation _worlddirection) (Class|PlayerController|DeprojectScreenPositiontoWorld _returnvalue_3 _returnvalue_2))
  ;[0.4463 0.5496 1] Controller Selection Test
  (:Pressed
    (bind _outhit (Collision|LineTraceByChannel _worldlocation (Math|Vector|MakeVector (.x _worlddirection) (.y _worlddirection) -1e+03) "TraceTypeQuery1" false 0 "None"))))

(event Input|MouseEvents|RightMouseButton
  (params (Key :type Key%20Structure :default "None"))
  ;[1 1 1] Check if rotating firsr
  (:Pressed
    ;[1 1 1] Set unit target location
    (CallFunction|GetGridFormation (Variables|Selection|GetUnitSelection))))

(event Input|MouseEvents|MiddleMouseButton
  (params (Key :type Key%20Structure :default "None"))
  ;[0.06772 0.3853 1] Rotate
  (:Pressed
    (bind _output_get (Variables|View|SetIs%20Rotating true))
    (bind _output_get_2 (Variables|View|SetMouseRotPos (.LocationX (Game|Player|GetMousePosition (Game|GetPlayerController 0))))))
  (:Released
    (Variables|View|SetIs%20Rotating false)
    (Variables|View|SetRotAxis 0.0)
    (Variables|View|SetRotSpeed 0.0)))

(fn ConstructionScript)

(fn MoveCamera
  (bind _camera_pawn (Variables|Default|GetCamera%20Pawn))
  (bind _rotspeed (Variables|View|GetRotSpeed))
  (bind _returnvalue (Transformation|GetActorRotation _camera_pawn))
  (bind _returnvalue_2 (* _rotspeed 0.005))
  (bind _returnvalue_3 (Math|Float|Clamp(Float) _returnvalue_2 -2.0 2.0))
  (bind _returnvalue_4 (+ (.yaw _returnvalue) _returnvalue_3))
  (bind _returnvalue_5 (Math|Rotator|MakeRotator 0.0 0.0 _returnvalue_4))
  (Class|WidgetLayoutLibrary|GetMousePositiononViewport)
  (bind _asbp_camera (Utilities|Casting|CastToBP_Camera (Variables|Default|GetCamera%20Pawn)))
  (bind _output_get (Variables|Movement|SetMove%20Speed (Math|Float|Clamp(Float) (/ (+ 1e+01 (Variables|/Script/Engine.SpringArmComponent|GetTargetArmLength (Variables|/Game/TopDown/BP_Camera.BP_Camera_C|GetSpringArm _asbp_camera))) 1.5e+02) 1e+01 64.0)))
  (Transformation|SetActorLocationAndRotation (Variables|Default|GetCamera%20Pawn) (+ (Transformation|GetActorLocation (Variables|Default|GetCamera%20Pawn)) (* (Math|Vector|Normalize (Math|Vector|RotateVector (Variables|Movement|GetMoveDir) (Math|Rotator|MakeRotator 0.0 0.0 (.yaw _returnvalue_5)))) _output_get)) (Math|Rotator|MakeRotator 0.0 0.0 (.yaw _returnvalue_5)))
  (Variables|View|SetRotPosCurrent 0.0)
  (bind _asbp_camera_2 (Utilities|Casting|CastToBP_Camera (Variables|Default|GetCamera%20Pawn)))
  (Variables|/Script/Engine.SpringArmComponent|SetTargetArmLength (Variables|/Game/TopDown/BP_Camera.BP_Camera_C|GetSpringArm _asbp_camera_2) (+ (Variables|View|GetCameraZoom) (Variables|/Script/Engine.SpringArmComponent|GetTargetArmLength (Variables|/Game/TopDown/BP_Camera.BP_Camera_C|GetSpringArm _asbp_camera_2)))))

(fn ResetRotationController
  (Variables|View|SetRotAxis 0.0)
  (Variables|View|SetRotAccelTime 0.0)
  (Variables|View|SetRotSpeed 0.0)
  (Variables|View|SetRotAccel 0.0))

(fn RotateCameraController
  (params (RotAxis :type Float%20%28double-precision%29))
  (bind _output_get (Variables|View|SetRotAccelTime (+ (Variables|View|GetRotAccelTime) 0.2)))
  (bind _output_get_2 (Variables|View|SetRotAxis RotAxis))
  (Variables|View|SetRotSpeed (* 3.0 (* _output_get_2 -1.0 (Variables|View|GetRotAccel))))
  (Variables|View|SetRotAccel (Math|Interpolation|Ease "EaseIn" 4.0 0.0 _output_get 2.0)))

(fn GetInputs
  (params (self2 :type Enhanced%20Input%20Subsystem%20Interface%20Interface))
  (Input|AddMappingContext self2 "/Game/Controls/Input/AC_Input.AC_Input" 0 "(bIgnoreAllPressedKeysUntilRelease=True,bForceImmediately=False,bNotifyUserSettings=False)")
  (Variables|Default|SetCamera%20Pawn (Game|Player|GetPlayerPawn 0))
  (Actor|GetActorOfClass "/Script/Landscape.Landscape")
  (Input|SetInputModeGameandUI self 0 "LockAlways" false false))

(fn AddUnittoSelectiom
  (params (UnitBase :type BP%20Unit%20Base%20Object%20Reference))
  (Utilities|Array|AddUnique (Variables|Selection|GetUnitSelection) UnitBase)
  (Default|IsSelected UnitBase true))

(fn RemoveUnitfromSelection
  (params (Unit :type BP%20Unit%20Base%20Object%20Reference))
  (Utilities|Array|RemoveItem (Variables|Selection|GetUnitSelection) Unit)
  (Default|IsSelected Unit false))

(fn ClearUnitSelection
  (bind _unitselection (Variables|Selection|GetUnitSelection))
  (for _array_element _unitselection
    (Default|IsSelected _array_element false))
  (Utilities|Array|Clear _unitselection))

(fn GetGridFormation
  (params (UNITS%20Selection :type Array%20of%20BP%20Unit%20Base%20Object%20References))
  (bind _returnvalue (Utilities|Array|Length UNITS%20Selection))
  (bind _hitresult (Game|Player|GetHitResultUnderCursorbyChannel "TraceTypeQuery1" true))
  (bind _rowarray (Variables|GridFormation|GetRowArray))
  (bind _col_array (Variables|GridFormation|Getcol%20array))
  (bind _unit_position_offset (Variables|GridFormation|GetUnit%20position%20offset))
  (bind _remainderarray (Variables|GridFormation|Getremainderarray))
  (bind _unit_position_offset_2 (Variables|GridFormation|GetUnit%20position%20offset))
  (bind _returnvalue_2 (Math|Conversions|ToFloat(Integer) _returnvalue))
  (bind _returnvalue_3 (Math|Conversions|ToFloat(Integer) _returnvalue))
  (bind (_x _y _z) (Math|Vector|BreakVector (.location _hitresult)))
  (bind _returnvalue_4 (Math|Float|Sqrt _returnvalue_2))
  (bind _returnvalue_5 (Math|Float|Ceil _returnvalue_4))
  (bind _returnvalue_6 (Math|Conversions|ToFloat(Integer) _returnvalue_5))
  (bind (_remainder _returnvalue_7) (Math|Float|Division(WholeandRemainder) _returnvalue_3 _returnvalue_6))
  ;[1 1 1] Clear Array
  (Utilities|Array|Clear (Variables|GridFormation|GetNewUnitPos))
  (Utilities|Array|Resize _rowarray _returnvalue_7)
  (Utilities|Array|Resize _col_array _returnvalue_5)
  (for (_ _array_index) _rowarray
    (for (_ _array_index_2) _col_array
      (Utilities|Array|Add (Variables|GridFormation|GetNewUnitPos) (Math|Vector|MakeVector (+ _x (Math|Conversions|ToFloat(Integer) (* _array_index_2 _unit_position_offset_2))) (+ (* _array_index _unit_position_offset_2) _y) _z)))
    (Utilities|Array|Resize _remainderarray (Math|Float|Ceil _remainder))
    (for (_ _array_index_3) _remainderarray
      (Utilities|Array|Add (Variables|GridFormation|GetNewUnitPos) (Math|Vector|MakeVector (+ _x (* _array_index_3 _unit_position_offset)) (+ _y (* _returnvalue_7 _unit_position_offset)) _z))))
  (for (_array_element _array_index_4) (Variables|Selection|GetUnitSelection)
    (AI|Components|Blackboard|SetValueasVector (AI|GetBlackboard _array_element) (Utilities|Name|MakeLiteralName "TargetLocation") (Utilities|Array|Get(acopy) (Variables|GridFormation|GetNewUnitPos) _array_index_4))))