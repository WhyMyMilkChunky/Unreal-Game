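; Base building Blueprint that randomizes its static mesh among three variants when play begins.
; BeginPlay calls NewFunction, which returns three booleans from random 1–3 checks, and applies the variant for the first true one.
; Each check rolls separately, so the variants are not equally likely and the mesh stays unchanged when all three fail.
; UpgradeTier is unused, and the construction script is empty.
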(event EventBeginPlay
  (bind (_returnvalue _returnvalue2 _returnvalue3) (CallFunction|NewFunction))
  (if _returnvalue
    (Components|StaticMesh|SetStaticMesh (Variables|Default|GetStaticMesh) (Variables|Building|GetBuilding%20Mesh%20Variant1))
    (elif _returnvalue2
      (Components|StaticMesh|SetStaticMesh (Variables|Default|GetStaticMesh) (Variables|Building|GetBuilding%20Mesh%20Variant2))
      (elif _returnvalue3
        (Components|StaticMesh|SetStaticMesh (Variables|Default|GetStaticMesh) (Variables|Building|GetBuilding%20Mesh%20Variant3))))))

(event Collision|EventActorBeginOverlap
  (params (OtherActor :type Actor%20Object%20Reference)))

(event EventTick
  (params (DeltaSeconds :type Float%20%28single-precision%29)))

(fn ConstructionScript)

(fn NewFunction
  (bind _returnvalue (Math|Random|RandomIntegerinRange 1 3))
  (return (== _returnvalue 1) (== _returnvalue 2) (== _returnvalue 3)))