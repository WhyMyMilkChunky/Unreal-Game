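; BP_MapBounds is a map boundary trigger that repositions the BP_Camera player pawn when something overlaps its AreaTrigger.
; BeginPlay caches the camera pawn, and MoveX and MoveY select which axes move toward the trigger's location plus Offset, preserving Z.
; The move is a single VInterpTo and SetActorLocation call per begin overlap, not a per-tick update.
; End overlap does nothing, and its "left bounds" debug print is disconnected.
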(event OnComponentBeginOverlap(AreaTrigger)
  (params (OverlappedComponent :type Primitive%20Component%20Object%20Reference) (OtherActor :type Actor%20Object%20Reference) (OtherComp :type Primitive%20Component%20Object%20Reference) (OtherBodyIndex :type Integer) (bFromSweep :type Boolean) (SweepResult :type Hit%20Result%20Structure%20%28by%20ref%29))
  (bind _playercamera (Variables|Default|GetPlayerCamera))
  (bind _areatrigger (Variables|Default|GetAreaTrigger))
  (bind _offset (Variables|Default|GetOffset))
  (bind _playercamera_2 (Variables|Default|GetPlayerCamera))
  (bind _playercamera_3 (Variables|Default|GetPlayerCamera))
  (bind _returnvalue (Transformation|GetWorldLocation _areatrigger))
  (bind _rootcomponent (Variables|/Script/Engine.Actor|GetRootComponent _playercamera))
  (bind _rootcomponent_2 (Variables|/Script/Engine.Actor|GetRootComponent _playercamera_2))
  (bind _rootcomponent_3 (Variables|/Script/Engine.Actor|GetRootComponent _playercamera_3))
  (bind _returnvalue_2 (Transformation|GetWorldLocation _rootcomponent_2))
  (bind _returnvalue_3 (Transformation|GetWorldLocation _rootcomponent_3))
  (bind _returnvalue_4 (Transformation|GetWorldLocation _rootcomponent))
  (bind _returnvalue_5 (+ _returnvalue _offset))
  (if (!= OtherActor self)
    (Utilities|Casting|CastToBP_Camera (Game|Player|GetPlayerPawn 0))
    ;[1 0 0.02972] Movement for both X and Y (IDK who the hell would need this but here)
    (if (and (Variables|Default|GetMoveX) (Variables|Default|GetMoveY))
      (Transformation|SetActorLocation (Variables|Default|GetPlayerCamera) (Math|Interpolation|VInterpTo (Math|Vector|MakeVector (.x _returnvalue_3) (.y _returnvalue_3) (.z _returnvalue_3)) (Math|Vector|MakeVector (.x _returnvalue_5) (.y _returnvalue_5) (.z _returnvalue_3)) (Utilities|Time|GetWorldDeltaSeconds) 0.0) false false)
      (else
        ;[1 0.1577 0.2141] Moves for X axis
        (if (Variables|Default|GetMoveX)
          (Transformation|SetActorLocation (Variables|Default|GetPlayerCamera) (Math|Interpolation|VInterpTo (Math|Vector|MakeVector (.x _returnvalue_2) (.y _returnvalue_2) (.z _returnvalue_2)) (Math|Vector|MakeVector (.x (+ (Transformation|GetWorldLocation (Variables|Default|GetAreaTrigger)) (Variables|Default|GetOffset))) (.y _returnvalue_2) (.z _returnvalue_2)) (Utilities|Time|GetWorldDeltaSeconds) 0.0) false false)
          (else
            ;[0 0.8842 1] Moves for Y axis
            (if (Variables|Default|GetMoveY)
              (Transformation|SetActorLocation (Variables|Default|GetPlayerCamera) (Math|Interpolation|VInterpTo (Math|Vector|MakeVector (.x _returnvalue_4) (.y _returnvalue_4) (.z _returnvalue_4)) (Math|Vector|MakeVector (.x _returnvalue_4) (.y (+ (Transformation|GetWorldLocation (Variables|Default|GetAreaTrigger)) (Variables|Default|GetOffset))) (.z _returnvalue_4)) (Utilities|Time|GetWorldDeltaSeconds) 0.0) false false))))))))

(event OnComponentEndOverlap(AreaTrigger)
  (params (OverlappedComponent :type Primitive%20Component%20Object%20Reference) (OtherActor :type Actor%20Object%20Reference) (OtherComp :type Primitive%20Component%20Object%20Reference) (OtherBodyIndex :type Integer))
  ;[0.1367 0.1406 0.06114] Garbage DEBUG RAAAAAAH
)

(event EventBeginPlay
  ;[0.408 0.2102 0.179] Shit Ass Dookie Balls pt.3
  (bind _asbp_camera (Utilities|Casting|CastToBP_Camera (Game|Player|GetPlayerPawn 0)))
  (Variables|Default|SetPlayerCamera _asbp_camera))

(event Collision|EventActorBeginOverlap
  (params (OtherActor :type Actor%20Object%20Reference)))

(event EventTick
  (params (DeltaSeconds :type Float%20%28single-precision%29))
  ;[0.408 0.2102 0.179] Shit Ass Dookie Balls pt.3
)

(fn ConstructionScript)