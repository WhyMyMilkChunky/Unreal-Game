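; Calendar actor that runs a timed month cycle, updates HUD year progress and calls EndOfYear on the game mode at rollover.
; Tick counts seconds per month, then AdvanceDate increments MonthIndex and toggles snow and rain particles on the camera; leaf logic is disconnected.
; MonthIndex selects the season, whose fog and foliage colours ease in through incremental per-frame lerps fed to BP_RetroPostProcess and the SeasonMaterials parameter collection.
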(event EventBeginPlay
  (bind _returnvalue (Actor|GetActorOfClass "/Game/RetroShadersV4/RetroShader/BP_RetroPostProcess.BP_RetroPostProcess_C"))
  (Variables|Default|SetPost%20Processing%20Bp _returnvalue)
  (bind _asin_game_mode (Utilities|Casting|CastToInGameMode (Game|GetGameMode)))
  (Variables|Default|SetAs%20in%20Game%20Mode _asin_game_mode)
  (bind _asbp_camera (Utilities|Casting|CastToBP_Camera (Game|Player|GetPlayerPawn 0)))
  (Variables|Default|SetAs%20BP%20Camera _asbp_camera)
  (Variables|Time|SetYearTotalTime (* (Variables|Time|GetSeconds%20per%20month) 12.0)))

(event Collision|EventActorBeginOverlap
  (params (OtherActor :type Actor%20Object%20Reference)))

(event EventTick
  (params (DeltaSeconds :type Float%20%28single-precision%29))
  (bind _returnvalue (Utilities|Time|GetWorldDeltaSeconds))
  (bind _returnvalue_2 (Utilities|Time|GetWorldDeltaSeconds))
  (bind _returnvalue_3 (Utilities|Time|GetWorldDeltaSeconds))
  (bind _returnvalue_4 (Utilities|Time|GetWorldDeltaSeconds))
  (bind _seconds_per_month (Variables|Time|GetSeconds%20per%20month))
  (bind _seconds_per_month_2 (Variables|Time|GetSeconds%20per%20month))
  (bind _seconds_per_month_3 (Variables|Time|GetSeconds%20per%20month))
  (bind _seconds_per_month_4 (Variables|Time|GetSeconds%20per%20month))
  (bind _returnvalue_5 (/ _returnvalue_2 _seconds_per_month))
  (bind _returnvalue_6 (/ _returnvalue_3 _seconds_per_month_3))
  (bind _returnvalue_7 (/ _returnvalue_4 _seconds_per_month_2))
  (bind _returnvalue_8 (/ _returnvalue _seconds_per_month_4))
  (Utilities|FlowControl|Sequence
    (:then_0
      ;[1 0.3444 0.8431] month timer
      (Variables|Time|SetTotalSecondsTimer (+ (Variables|Time|GetTotalSecondsTimer) (Utilities|Time|GetWorldDeltaSeconds)))
      (bind _iscountingover (CallFunction|CalculateSeconds (Variables|Time|GetSeconds%20per%20month)))
      (Default|CalculateProgresstoEndOfYear (Variables|/Game/Blueprints/InGameMode.InGameMode_C|GetAs%20HUD%20Canvas (Variables|Default|GetAs%20in%20Game%20Mode)) (Variables|Time|GetTotalSecondsTimer) (Variables|Time|GetYearTotalTime) (Variables|Time|GetMonthIndex))
      (if _iscountingover
        (Variables|Time|SetSeconds 0.0)
        (Utilities|FlowControl|DelayUntilNextTick)
        (CallFunction|AdvanceDate)))
    (:then_1
      ;[1 1 1] Winter
      (if (Math|Integer|InRange(Integer) (Variables|Time|GetMonthIndex) 0 2)
        (Default|SetColoursfromSeasons (Variables|Default|GetPost%20Processing%20Bp) (Math|Color|Lerp(LinearColor) (Variables|Default|GetLast%20FogFarColor) "(R=0.301961,G=0.313726,B=0.478431,A=1.000000)" _returnvalue_8) (Math|Color|Lerp(LinearColor) (Variables|Default|GetLast%20FogCloseColor) "(R=0.760784,G=0.792157,B=1.000000,A=1.000000)" _returnvalue_8))
        (Variables|Default|SetLast%20FogFarColor (Math|Color|Lerp(LinearColor) (Variables|Default|GetLast%20FogFarColor) "(R=0.301961,G=0.313726,B=0.478431,A=1.000000)" _returnvalue_8))
        (Variables|Default|SetLast%20FogCloseColor (Math|Color|Lerp(LinearColor) (Variables|Default|GetLast%20FogCloseColor) "(R=0.760784,G=0.792157,B=1.000000,A=1.000000)" _returnvalue_8))
        (Rendering|Material|SetVectorParameterValue "/Game/Map/Landscape/Foliage/SeasonMaterials.SeasonMaterials" "Foliage Colour" (Math|Color|Lerp(LinearColor) (Variables|Colours|GetLast%20Primary%20Colour) (Variables|Colours|GetWinter) _returnvalue_8) :!class /Script/Engine.KismetMaterialLibrary)
        (Variables|Colours|SetLast%20Primary%20Colour (Math|Color|Lerp(LinearColor) (Variables|Colours|GetLast%20Primary%20Colour) (Variables|Colours|GetWinter) _returnvalue_8))
        (Rendering|Material|SetVectorParameterValue "/Game/Map/Landscape/Foliage/SeasonMaterials.SeasonMaterials" "Foliage Secondary Colour" (Math|Color|Lerp(LinearColor) (Variables|Colours|GetLast%20Secondary%20Colour) "(R=0.128898,G=0.244792,B=0.077772,A=1.000000)" (/ (Utilities|Time|GetWorldDeltaSeconds) (Variables|Time|GetSeconds%20per%20month))) :!class /Script/Engine.KismetMaterialLibrary)
        (Variables|Colours|SetLast%20Secondary%20Colour (Math|Color|Lerp(LinearColor) (Variables|Colours|GetLast%20Secondary%20Colour) "(R=0.128898,G=0.244792,B=0.077772,A=1.000000)" (/ (Utilities|Time|GetWorldDeltaSeconds) (Variables|Time|GetSeconds%20per%20month))))
        (else
          ;[1 1 1] Spring
          (if (Math|Integer|InRange(Integer) (Variables|Time|GetMonthIndex) 3 5)
            (Default|SetColoursfromSeasons (Variables|Default|GetPost%20Processing%20Bp) (Math|Color|Lerp(LinearColor) (Variables|Default|GetLast%20FogFarColor) "(R=0.270588,G=0.360784,B=0.380392,A=1.000000)" _returnvalue_6) (Math|Color|Lerp(LinearColor) (Variables|Default|GetLast%20FogCloseColor) "(R=0.282353,G=0.196078,B=0.082353,A=1.000000)" _returnvalue_6))
            (Variables|Default|SetLast%20FogFarColor (Math|Color|Lerp(LinearColor) (Variables|Default|GetLast%20FogFarColor) "(R=0.270588,G=0.360784,B=0.380392,A=1.000000)" _returnvalue_6))
            (Variables|Default|SetLast%20FogCloseColor (Math|Color|Lerp(LinearColor) (Variables|Default|GetLast%20FogCloseColor) "(R=0.282353,G=0.196078,B=0.082353,A=1.000000)" _returnvalue_6))
            (Rendering|Material|SetVectorParameterValue "/Game/Map/Landscape/Foliage/SeasonMaterials.SeasonMaterials" "Foliage Colour" (Math|Color|Lerp(LinearColor) (Variables|Colours|GetLast%20Primary%20Colour) (Variables|Colours|GetSpring%20Color) _returnvalue_6) :!class /Script/Engine.KismetMaterialLibrary)
            (Variables|Colours|SetLast%20Primary%20Colour (Math|Color|Lerp(LinearColor) (Variables|Colours|GetLast%20Primary%20Colour) (Variables|Colours|GetSpring%20Color) _returnvalue_6))
            (Rendering|Material|SetVectorParameterValue "/Game/Map/Landscape/Foliage/SeasonMaterials.SeasonMaterials" "Foliage Secondary Colour" (Math|Color|Lerp(LinearColor) (Variables|Colours|GetLast%20Secondary%20Colour) "(R=0.050240,G=0.145833,B=0.022300,A=1.000000)" (/ (Utilities|Time|GetWorldDeltaSeconds) (Variables|Time|GetSeconds%20per%20month))) :!class /Script/Engine.KismetMaterialLibrary)
            (Variables|Colours|SetLast%20Secondary%20Colour (Math|Color|Lerp(LinearColor) (Variables|Colours|GetLast%20Secondary%20Colour) "(R=0.050240,G=0.145833,B=0.022300,A=1.000000)" (/ (Utilities|Time|GetWorldDeltaSeconds) (Variables|Time|GetSeconds%20per%20month))))
            (else
              ;[1 1 1] Summer
              (if (Math|Integer|InRange(Integer) (Variables|Time|GetMonthIndex) 6 8)
                (Default|SetColoursfromSeasons (Variables|Default|GetPost%20Processing%20Bp) (Math|Color|Lerp(LinearColor) (Variables|Default|GetLast%20FogFarColor) "(R=0.219608,G=0.282353,B=0.329412,A=1.000000)" _returnvalue_7) (Math|Color|Lerp(LinearColor) (Variables|Default|GetLast%20FogCloseColor) "(R=0.211765,G=0.125490,B=0.027451,A=1.000000)" _returnvalue_7))
                (Variables|Default|SetLast%20FogFarColor (Math|Color|Lerp(LinearColor) (Variables|Default|GetLast%20FogFarColor) "(R=0.219608,G=0.282353,B=0.329412,A=1.000000)" _returnvalue_7))
                (Variables|Default|SetLast%20FogCloseColor (Math|Color|Lerp(LinearColor) (Variables|Default|GetLast%20FogCloseColor) "(R=0.211765,G=0.125490,B=0.027451,A=1.000000)" _returnvalue_7))
                (Rendering|Material|SetVectorParameterValue "/Game/Map/Landscape/Foliage/SeasonMaterials.SeasonMaterials" "Foliage Colour" (Math|Color|Lerp(LinearColor) (Variables|Colours|GetLast%20Primary%20Colour) (Variables|Colours|GetSummer) _returnvalue_7) :!class /Script/Engine.KismetMaterialLibrary)
                (Variables|Colours|SetLast%20Primary%20Colour (Math|Color|Lerp(LinearColor) (Variables|Colours|GetLast%20Primary%20Colour) (Variables|Colours|GetSummer) _returnvalue_7))
                (Rendering|Material|SetVectorParameterValue "/Game/Map/Landscape/Foliage/SeasonMaterials.SeasonMaterials" "Foliage Secondary Colour" (Math|Color|Lerp(LinearColor) (Variables|Colours|GetLast%20Secondary%20Colour) "(R=0.171845,G=0.192708,B=0.017063,A=1.000000)" (/ (Utilities|Time|GetWorldDeltaSeconds) (Variables|Time|GetSeconds%20per%20month))) :!class /Script/Engine.KismetMaterialLibrary)
                (Variables|Colours|SetLast%20Secondary%20Colour (Math|Color|Lerp(LinearColor) (Variables|Colours|GetLast%20Secondary%20Colour) "(R=0.171845,G=0.192708,B=0.017063,A=1.000000)" (/ (Utilities|Time|GetWorldDeltaSeconds) (Variables|Time|GetSeconds%20per%20month))))
                (else
                  ;[1 1 1] Fall
                  (if (Math|Integer|InRange(Integer) (Variables|Time|GetMonthIndex) 9 11)
                    (Default|SetColoursfromSeasons (Variables|Default|GetPost%20Processing%20Bp) (Math|Color|Lerp(LinearColor) (Variables|Default|GetLast%20FogFarColor) "(R=0.301961,G=0.247059,B=0.207843,A=1.000000)" _returnvalue_5) (Math|Color|Lerp(LinearColor) (Variables|Default|GetLast%20FogCloseColor) "(R=0.454902,G=0.313726,B=0.298039,A=1.000000)" _returnvalue_5))
                    (Variables|Default|SetLast%20FogFarColor (Math|Color|Lerp(LinearColor) (Variables|Default|GetLast%20FogFarColor) "(R=0.301961,G=0.247059,B=0.207843,A=1.000000)" _returnvalue_5))
                    (Variables|Default|SetLast%20FogCloseColor (Math|Color|Lerp(LinearColor) (Variables|Default|GetLast%20FogCloseColor) "(R=0.454902,G=0.313726,B=0.298039,A=1.000000)" _returnvalue_5))
                    (Rendering|Material|SetVectorParameterValue "/Game/Map/Landscape/Foliage/SeasonMaterials.SeasonMaterials" "Foliage Colour" (Math|Color|Lerp(LinearColor) (Variables|Colours|GetLast%20Primary%20Colour) (Variables|Colours|GetFall) _returnvalue_5) :!class /Script/Engine.KismetMaterialLibrary)
                    (Variables|Colours|SetLast%20Primary%20Colour (Math|Color|Lerp(LinearColor) (Variables|Colours|GetLast%20Primary%20Colour) (Variables|Colours|GetFall) _returnvalue_5))
                    (Rendering|Material|SetVectorParameterValue "/Game/Map/Landscape/Foliage/SeasonMaterials.SeasonMaterials" "Foliage Secondary Colour" (Math|Color|Lerp(LinearColor) (Variables|Colours|GetLast%20Secondary%20Colour) (Variables|Colours|GetWinter) (/ (Utilities|Time|GetWorldDeltaSeconds) (Variables|Time|GetSeconds%20per%20month))) :!class /Script/Engine.KismetMaterialLibrary)
                    (Variables|Colours|SetLast%20Secondary%20Colour (Math|Color|Lerp(LinearColor) (Variables|Colours|GetLast%20Secondary%20Colour) (Variables|Colours|GetWinter) (/ (Utilities|Time|GetWorldDeltaSeconds) (Variables|Time|GetSeconds%20per%20month))))))))))))))

(fn ConstructionScript)

(fn AdvanceDate
  (if (> (Variables|Time|GetMonthIndex) (- (Utilities|Array|Length (Variables|Time|GetMonths)) 1))
    ;[1 0.2199 0.9465] reset month and end year
    (Variables|Time|SetMonthIndex 0)
    (Default|EndOfYear (Variables|Default|GetAs%20in%20Game%20Mode))
    (else
      ;[1 0.3585 0.9743] increment month
      (bind _result (Math|Integer|IncrementInt (Variables|Time|GetMonthIndex))
        (:%20%20
          (Variables|Time|SetMonthIndex _result)
          ;[0.1039 0.1866 1] Particles
          (Utilities|FlowControl|Sequence
            (:then_0
              ;;[1 1 1] Adds Snow For December - February
              (if (< (Variables|Time|GetMonthIndex) 3)
                (Default|ActivateParticle (Variables|Default|GetAs%20BP%20Camera) true (Variables|/Game/Actors/Player/BP_Camera.BP_Camera_C|GetFXS_Snow_System (Variables|Default|GetAs%20BP%20Camera)))
                (else
                  (Default|ActivateParticle (Variables|Default|GetAs%20BP%20Camera) false (Variables|/Game/Actors/Player/BP_Camera.BP_Camera_C|GetFXS_Snow_System (Variables|Default|GetAs%20BP%20Camera))))))
            (:then_2
              ;;[1 1 1] Adds Rain For April
              (if (== (Variables|Time|GetMonthIndex) 4)
                (Default|ActivateParticle (Variables|Default|GetAs%20BP%20Camera) true (Variables|/Game/Actors/Player/BP_Camera.BP_Camera_C|GetFXS_Rain_System (Variables|Default|GetAs%20BP%20Camera)))
                (else
                  (Default|ActivateParticle (Variables|Default|GetAs%20BP%20Camera) false (Variables|/Game/Actors/Player/BP_Camera.BP_Camera_C|GetFXS_Rain_System (Variables|Default|GetAs%20BP%20Camera))))))))))))

(fn CalculateSeconds
  (params (Reset%20Count%20Amount :type Float%20%28double-precision%29))
  (bind _output_get (Variables|Time|SetSeconds (+ (Variables|Time|GetSeconds) (Utilities|Time|GetWorldDeltaSeconds))))
  (return _output_get (> _output_get Reset%20Count%20Amount)))