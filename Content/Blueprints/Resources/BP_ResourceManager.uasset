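; Resource manager actor that tracks quantities of each resource type and values of named statistics in two maps.
; BeginPlay seeds both maps at zero, re-seeding the statistics inside the resource enum loop.
; Functions add, subtract and read resources without bounds checks, add and read statistics, or replace the whole resource map.
; A test function grants random resource amounts and a fixed increase to every statistic.
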(event EventBeginPlay
  ;[1 1 1] For each resource, add to map
  (bind _enumvalue (|ForEachE_ResourceType)
    (:LoopBody
      (Utilities|Map|Add (Variables|Default|GetResources%20Map) _enumvalue 0)
      ;[1 1 1] for each statistcs add to map
      (for _array_element (Variables|Default|GetStatistics)
        (Utilities|Map|Add (Variables|Default|GetStatistics%20map) _array_element 0.0)))))

(event Collision|EventActorBeginOverlap
  (params (OtherActor :type Actor%20Object%20Reference)))

(event EventTick
  (params (DeltaSeconds :type Float%20%28single-precision%29)))

(fn ConstructionScript)

(fn AddResource
  (params (AmountAdded :type Integer) (Resource :type E_ResourceType%20Enum :default "NewEnumerator0"))
  (bind _resources_map (Variables|Default|GetResources%20Map))
  ;[1 1 1] Finds input resource and adds to map
  (Utilities|Map|Add _resources_map Resource (+ (.Value (Utilities|Map|Find _resources_map Resource)) AmountAdded))
  ;[1 1 1] Update UI event called
  (return Resource))

(fn GetResource
  (params (Find%20Resource :type E_ResourceType%20Enum :default "NewEnumerator0"))
  (return Find%20Resource (.Value (Utilities|Map|Find (Variables|Default|GetResources%20Map) Find%20Resource))))

(fn SubtractResouce
  (params (ResourceChanged :type E_ResourceType%20Enum :default "NewEnumerator0") (Quantity :type Integer))
  ;[1 1 1] Finds input resource and adds to map
  (Utilities|Map|Add (Variables|Default|GetResources%20Map) ResourceChanged (- (.Value (Utilities|Map|Find (Variables|Default|GetResources%20Map) ResourceChanged)) Quantity))
  (return ResourceChanged))

(fn AddResourcesTEST
  (bind _enumvalue (|ForEachE_ResourceType)
    (:LoopBody
      (Resource|AddResource (Math|Random|RandomIntegerinRange 5 12) _enumvalue))
    (:then
      (for _array_element (Variables|Default|GetStatistics)
        (Stats|AddStatistic 5.0 _array_element)))))

(fn AddStatistic
  (params (AmountAdded :type Float%20%28double-precision%29) (Statistic :type E_Statistics%20Enum :default "NewEnumerator0"))
  (bind _statistics_map (Variables|Default|GetStatistics%20map))
  ;[1 1 1] Finds input resource and adds to map
  (Utilities|Map|Add _statistics_map Statistic (+ (.Value (Utilities|Map|Find _statistics_map Statistic)) AmountAdded))
  (return Statistic))

(fn GetStatistic
  (params (Find%20Resource :type E_Statistics%20Enum :default "NewEnumerator0"))
  (return Find%20Resource (.Value (Utilities|Map|Find (Variables|Default|GetStatistics%20map) Find%20Resource))))

(fn UpdateResourceMap
  (params (New%20Resource%20map :type Map%20of%20E_ResourceType%20Enums%20to%20Integers :default "NewEnumerator0"))
  (Variables|Default|SetResources%20Map New%20Resource%20map))