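; NewGameMode holds the game's resource totals for wood, iron, gold and stone.
; Each Add function updates a count and passes the new value to a matching Collected call, which appears to be an event dispatcher.
; AddGold and AddStone compute their totals from IronCount rather than their own counts, so those totals do not accumulate independently.
; Event graph and construction script are empty.
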(event EventBeginPlay)

(event EventTick
  (params (DeltaSeconds :type Float%20%28single-precision%29)))

(fn ConstructionScript)

(fn AddWood
  (params (#OfWood :type Integer))
  (bind _output_get (Variables|Default|SetWoodCount (+ (Variables|Default|GetWoodCount) #OfWood)))
  (Default|CallWoodCollected _output_get))

(fn AddIron
  (params (#OfIron :type Integer))
  (bind _output_get (Variables|Default|SetIronCount (+ (Variables|Default|GetIronCount) #OfIron)))
  (Default|CallIronCollected _output_get))

(fn AddGold
  (params (#%20of%20Gold :type Integer))
  (bind _output_get (Variables|Default|SetGoldCount (+ (Variables|Default|GetIronCount) #%20of%20Gold)))
  (Default|CallGoldCollected _output_get))

(fn AddStone
  (params (#%20Of%20Stone :type Integer))
  (bind _output_get (Variables|Default|SetStoneCount (+ (Variables|Default|GetIronCount) #%20Of%20Stone)))
  (Default|CallStoneCollected _output_get))