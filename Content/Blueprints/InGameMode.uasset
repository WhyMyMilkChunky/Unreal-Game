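; In-game mode for a resource management game with population, happiness and a yearly gold quota.
; It caches the resource manager, calendar and HUD, mirroring resources into a local map for the UI.
; Tick totals food to nudge happiness and moves hover popups to the cursor, while month events grow population.
; Year end pauses for a quota result; helpers raise the quota and spawn knights, while screen fading is unwired.
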(event Custom|UpdateResourceUI
  ;[1 1 1] make array that iterates all
  (CallFunction|UpdateResources)
  (Default|SetGoldonQuoteHud (Variables|HUD|GetAs%20HUD%20Canvas)))

(event Custom|popup%20unhover
  ;[1 0.4618 0.8444] unhover popup
  (Widget|SetVisibility (Variables|HUD|Getrequired%20resource%20popup) "Hidden")
  (Widget|RemovefromParent (Variables|HUD|Getrequired%20resource%20popup)))

(event Custom|Required%20resourse%20popup
  ;[1 0.3356 0.8761] Building hover popup
  (bind _returnvalue (UserInterface|CreateWidget "/Game/HUD/Widget_Contents/WBP_HUD_RequiredResourceBox.WBP_HUD_RequiredResourceBox_C" 0 (Variables|Default|GetBuilding%20class) (Variables|HUD|GetBP_ResourceManager)))
  (bind _output_get (Variables|HUD|Setrequired%20resource%20popup _returnvalue))
  (Class|Widget|ForceVolatile _output_get true)
  (Class|UserWidget|SetDesiredSizeinViewport (Variables|HUD|Getrequired%20resource%20popup) "(X=300.000000,Y=300.000000)")
  (UserInterface|Viewport|AddtoViewport (Variables|HUD|Getrequired%20resource%20popup) 0))

(event Custom|CombatUnhover
  (Widget|SetVisibility (stale Custom|Combat%20Stats _output_get) "Hidden")
  (Widget|RemovefromParent (stale Custom|Combat%20Stats _output_get)))

(event Custom|Combat%20Stats
  (bind _returnvalue (UserInterface|CreateWidget "/Game/HUD/Widget_Contents/WBP_UnitPopup.WBP_UnitPopup_C"))
  (bind _output_get (Variables|Default|SetUnit%20Stats%20Popup _returnvalue))
  (Class|UserWidget|SetDesiredSizeinViewport _output_get "(X=300.000000,Y=300.000000)")
  (UserInterface|Viewport|AddtoViewport _output_get 0))

(event Custom|End%20Of%20Year
  ;[1 1 1] Checks if Quota is met
  (Game|SetGamePaused true)
  (Default|EndOfYearQuotaPopup (Variables|HUD|GetAs%20HUD%20Canvas) (>= (.Value (Utilities|Map|Find (Variables|Default|GetResource%20Map) "NewEnumerator7")) (Variables|Game|GetGold%20Quota)))
  ;;[1 0.3287 0.8674] increment the year
  (Math|Integer|IncrementInt (Variables|/Game/Blueprints/BP_CalendarSystem.BP_CalendarSystem_C|GetYear (Variables|Default|GetBp_Calendar))))

(event Custom|MonthPassEvent
  (CallFunction|PopulationUpdate))

(event Custom|FadeScreenOut)

(event EventBeginPlay
  ;[1 1 1] Set Variables
  (CallFunction|SetVariables)
  (Utilities|FlowControl|DelayUntilNextTick)
  (CallFunction|UpdateResourceUI))

(event EventTick
  (params (DeltaSeconds :type Float%20%28single-precision%29))
  (bind _returnvalue (Game|GetPlayerController 0))
  (bind _returnvalue_2 (Game|GetPlayerController 0))
  (bind _required_resource_popup (Variables|HUD|Getrequired%20resource%20popup))
  (bind _unit_stats_popup (Variables|Default|GetUnit%20Stats%20Popup))
  (bind (_locationx _locationy) (Game|Player|GetMousePosition _returnvalue))
  (bind (_locationx_2 _locationy_2) (Game|Player|GetMousePosition _returnvalue_2))
  ;[1 0 0.8527] Event Tick
  (Food|SetTotalFood)
  (CallFunction|CalculateHappiness)
  (if (Utilities|IsValid _required_resource_popup)
    (Class|UserWidget|SetPositioninViewport _required_resource_popup (Math|Vector2D|MakeVector2D _locationx _locationy) true)
    (if (Utilities|IsValid _unit_stats_popup)
      (Class|UserWidget|SetPositioninViewport _unit_stats_popup (Math|Vector2D|MakeVector2D _locationx_2 _locationy_2) false))))

(fn ConstructionScript)

(fn SetVariables
  (bind _returnvalue (Actor|GetActorOfClass "/Game/Blueprints/Resources/BP_ResourceManager.BP_ResourceManager_C"))
  (Variables|HUD|SetBP_ResourceManager _returnvalue)
  (bind _ashud_canvas (Utilities|Casting|CastToHUD_Canvas (HUD|GetHUD (Game|GetPlayerController 0))))
  (Variables|HUD|SetAs%20HUD%20Canvas _ashud_canvas)
  (Variables|Default|SetResource%20Map (Variables|/Game/Blueprints/Resources/BP_ResourceManager.BP_ResourceManager_C|GetResources%20Map (Variables|HUD|GetBP_ResourceManager)))
  (bind _returnvalue_2 (Actor|GetActorOfClass "/Game/Blueprints/BP_CalendarSystem.BP_CalendarSystem_C"))
  (Variables|Default|SetBp_Calendar _returnvalue_2))

(fn SpawnEnemies
  (params (EnemyAmount :type Integer))
  (bind _returnvalue (Game|GetPlayerController 0))
  (bind _hitresult (Game|Player|GetHitResultUnderCursorbyChannel _returnvalue "TraceTypeQuery5" false))
  (bind (_x _y _z) (Math|Vector|BreakVector (.location _hitresult)))
  (for _index (range 1 EnemyAmount)
    (bind _returnvalue_2 (Game|SpawnActorfromClass :Class "/Game/Actors/Combat/Group/Unit_EnemyKnight.Unit_EnemyKnight_C" :SpawnTransform (Math|Conversions|ToTransform(Vector) (Math|Vector|MakeVector 0.0 0.0 0.0)) :CollisionHandlingOverride "Undefined" :TransformScaleMethod "MultiplyWithRoot" :Instigator 0))
    (Transformation|SetActorLocation _returnvalue_2 (Math|Vector|MakeVector (+ (Math|Conversions|ToFloat(Integer) (* _index 100)) _x) _y (+ _z 1e+02)) false false)))

(fn QuotaResetandIncrease
  (Utilities|FlowControl|Sequence
    (:then_0
      ;[1 0.3217 0.8023] subtract quota from current gold
      (Default|SubtractResouce (Variables|HUD|GetBP_ResourceManager) "NewEnumerator7" (Variables|Game|GetGold%20Quota)))
    (:then_1
      ;[1 0.3364 0.806] Quota increase by percent
      (Variables|Game|SetGold%20Quota (Math|Float|Round (* (Variables|Game|GetGold%20Quota) (Variables|Game|GetQuota%20Increase%20multiply)))))
    (:then_2
      (CallFunction|UpdateResourceUI))))

(fn UpdateResources
  (bind _resource_map (Variables|Default|GetResource%20Map))
  ;[1 1 1] update resource manager for each resource
  (bind _keys (Utilities|Map|Keys (Variables|Default|GetResource%20Map)))
  (for _array_element _keys
    ;;[1 1 1] Remove and readd key with updated value
    (bind (_found_resource _quantity) (Default|GetResource (Variables|HUD|GetBP_ResourceManager) _array_element))
    (Utilities|Map|Remove _resource_map _found_resource)
    (Utilities|Map|Add _resource_map _found_resource _quantity)
    ;[1 1 1] update  resource menu Hud
    (Variables|/Game/Blueprints/HUD/WBP_HUD_ResourcesMenu.WBP_HUD_ResourcesMenu_C|SetResourceMap (Variables|/Game/Blueprints/HUD/WBP_HUD_InGame.WBP_HUD_InGame_C|GetWBP_HUD_ResourcesMenu (Variables|HUD|GetHudInGame)) (Variables|Default|GetResource%20Map))))

(fn TransitionScene
  (params (Map :type Name))
  (CallFunction|FadeScreenOut))

(fn PopulationUpdate
  (bind _bp_resourcemanager (Variables|HUD|GetBP_ResourceManager))
  (bind _statistics_map (Variables|/Game/Blueprints/Resources/BP_ResourceManager.BP_ResourceManager_C|GetStatistics%20map _bp_resourcemanager))
  (bind _value (Utilities|Map|Find _statistics_map "NewEnumerator0"))
  (if (!= _value (.Value (Utilities|Map|Find _statistics_map "NewEnumerator5")))
    (Default|AddStatistic (Variables|HUD|GetBP_ResourceManager) 2.0 "NewEnumerator0")
    (Development|PrintString (Utilities|String|ToString(Float) _value))))

(fn SetTotalFood
  (bind _resource_map (Variables|Default|GetResource%20Map))
  (Variables|Default|SettotalFood (+ (.Value (Utilities|Map|Find _resource_map "NewEnumerator13")) (.Value (Utilities|Map|Find _resource_map "NewEnumerator5")) (.Value (Utilities|Map|Find _resource_map "NewEnumerator9")))))

(fn CalculateHappiness
  (if (< (/ (Variables|Default|GettotalFood) (.Value (Utilities|Map|Find (Variables|/Game/Blueprints/Resources/BP_ResourceManager.BP_ResourceManager_C|GetStatistics%20map (Variables|HUD|GetBP_ResourceManager)) "NewEnumerator0"))) 1.0)
    (Default|AddStatistic (Variables|HUD|GetBP_ResourceManager) -0.001 "NewEnumerator1")
    (else
      (Default|AddStatistic (Variables|HUD|GetBP_ResourceManager) 0.001 "NewEnumerator1"))))