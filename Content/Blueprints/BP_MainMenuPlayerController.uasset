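; BP_MainMenuPlayerController is a main-menu player controller whose event graph only sets UI-only input on BeginPlay.
; It also contains RTS functions, not called from that event graph, for camera movement, unit selection, cursor-based grid formations and enemy targeting.
; Building helpers handle preview, rotation, popups and debris, with placement validated by five downward traces requiring landscape hits at bounds corners and center.
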(event EventBeginPlay
  (Input|SetInputModeUIOnly (Game|GetPlayerController 0) 0 "DoNotLock" false))

(fn ConstructionScript)

(fn MoveCamera
  (bind _returnvalue (Utilities|Time|GetWorldDeltaSeconds))
  (bind _camera_pawn (Variables|Default|GetCamera%20Pawn))
  (bind _rotspeed (Variables|View|GetRotSpeed))
  (bind _returnvalue_2 (Transformation|GetActorRotation _camera_pawn))
  (bind _returnvalue_3 (* _rotspeed 0.005))
  (bind _returnvalue_4 (Math|Float|Clamp(Float) _returnvalue_3 -2.0 2.0))
  (bind _returnvalue_5 (* _returnvalue_4 _returnvalue 1e+02))
  (bind _returnvalue_6 (+ (.yaw _returnvalue_2) _returnvalue_5))
  (bind _returnvalue_7 (Math|Rotator|MakeRotator 0.0 0.0 _returnvalue_6))
  (Class|WidgetLayoutLibrary|GetMousePositiononViewport)
  (bind _asbp_camera (Utilities|Casting|CastToBP_Camera (Variables|Default|GetCamera%20Pawn)))
  (bind _output_get (Variables|Movement|SetMove%20Speed (Math|Float|Clamp(Float) (/ (+ 1e+01 (Variables|/Script/Engine.SpringArmComponent|GetTargetArmLength (Variables|/Game/Actors/Player/BP_Camera.BP_Camera_C|GetSpringArm _asbp_camera))) 1.5e+02) 1e+01 64.0)))
  (Transformation|SetActorLocationAndRotation (Variables|Default|GetCamera%20Pawn) (+ (Transformation|GetActorLocation (Variables|Default|GetCamera%20Pawn)) (* (Math|Vector|Normalize (Math|Vector|RotateVector (Variables|Movement|GetMoveDir) (Math|Rotator|MakeRotator 0.0 0.0 (.yaw _returnvalue_7)))) (* _output_get (Utilities|Time|GetWorldDeltaSeconds) 1e+02))) (Math|Rotator|MakeRotator 0.0 0.0 (.yaw _returnvalue_7)))
  (Variables|View|SetRotPosCurrent 0.0)
  ;[1 1 1] Limits Camera Zoom ( Adjust Values to Change Limit (Curr Min:1000 Max:10000))
  (bind _asbp_camera_2 (Utilities|Casting|CastToBP_Camera (Variables|Default|GetCamera%20Pawn)))
  (bind _output_get_2 (Variables|/Script/Engine.SpringArmComponent|SetTargetArmLength (Variables|/Game/Actors/Player/BP_Camera.BP_Camera_C|GetSpringArm _asbp_camera_2) (Math|Float|Clamp(Float) (+ (Variables|View|GetCameraZoom) (Variables|/Script/Engine.SpringArmComponent|GetTargetArmLength (Variables|/Game/Actors/Player/BP_Camera.BP_Camera_C|GetSpringArm _asbp_camera_2))) 1e+03 1e+04)))
  (bind _output_get_3 (Variables|Camera|SetTAL _output_get_2))
  (Transformation|SetRelativeLocation (Variables|/Game/Actors/Player/BP_Camera.BP_Camera_C|GetMinimapSA _asbp_camera_2) (Math|Vector|MakeVector _output_get_3 0.0 0.0) false false))

(fn ResetRotationController
  (Variables|View|SetRotAxis 0.0)
  (Variables|View|SetRotAccelTime 0.0)
  (Variables|View|SetRotSpeed 0.0)
  (Variables|View|SetRotAccel 0.0))

(fn RotateCameraController
  (params (RotAxis :type Float%20%28double-precision%29))
  (bind _output_get (Variables|View|SetRotAccelTime (+ (Variables|View|GetRotAccelTime) 0.2)))
  (bind _output_get_2 (Variables|View|SetRotAxis RotAxis))
  (Variables|View|SetRotSpeed (* 3.0 (* _output_get_2 -1.0 (Variables|View|GetRotAccel))))
  (Variables|View|SetRotAccel (Math|Interpolation|Ease "EaseIn" 4.0 0.0 _output_get 2.0)))

(fn GetInputs
  (params (self2 :type Enhanced%20Input%20Subsystem%20Interface%20Interface))
  (Input|AddMappingContext self2 "/Game/Controls/Input/AC_Input.AC_Input" 0 "(bIgnoreAllPressedKeysUntilRelease=True,bForceImmediately=False,bNotifyUserSettings=False)")
  (Variables|Default|SetCamera%20Pawn (Game|Player|GetPlayerPawn 0))
  (Actor|GetActorOfClass "/Script/Landscape.Landscape")
  (Input|SetInputModeGameandUI self 0 "LockAlways" false false))

(fn AddUnittoSelectiom
  (params (UnitBase :type BP%20Unit%20Base%20Object%20Reference))
  (if (not (Variables|/Game/Actors/Combat/Group/BP_UnitBase.BP_UnitBase_C|GetIsEnemy UnitBase))
    (Utilities|Array|AddUnique (Variables|Selection|GetUnitSelection) UnitBase)
    (Default|IsSelected UnitBase true)))

(fn RemoveUnitfromSelection
  (params (Unit :type BP%20Unit%20Base%20Object%20Reference))
  (Utilities|Array|RemoveItem (Variables|Selection|GetUnitSelection) Unit)
  (Default|IsSelected Unit false))

(fn ClearUnitSelection
  (bind _unitselection (Variables|Selection|GetUnitSelection))
  (for _array_element _unitselection
    (Default|IsSelected _array_element false))
  (Utilities|Array|Clear _unitselection))

(fn GetGridFormation
  (params (UNITS%20Selection :type Array%20of%20BP%20Unit%20Base%20Object%20References))
  (bind _returnvalue (Utilities|Array|Length UNITS%20Selection))
  (bind _hitresult (Game|Player|GetHitResultUnderCursorbyChannel "TraceTypeQuery5" true))
  (bind _rowarray (Variables|GridFormation|GetRowArray))
  (bind _newunitpos (Variables|GridFormation|GetNewUnitPos))
  (bind _col_array (Variables|GridFormation|Getcol%20array))
  (bind _unit_position_offset (Variables|GridFormation|GetUnit%20position%20offset))
  (bind _remainderarray (Variables|GridFormation|Getremainderarray))
  (bind _unit_position_offset_2 (Variables|GridFormation|GetUnit%20position%20offset))
  (bind _returnvalue_2 (Math|Conversions|ToFloat(Integer) _returnvalue))
  (bind _returnvalue_3 (Math|Conversions|ToFloat(Integer) _returnvalue))
  (bind (_x _y _z) (Math|Vector|BreakVector (.location _hitresult)))
  (bind _returnvalue_4 (Math|Float|Sqrt _returnvalue_2))
  (bind _returnvalue_5 (Math|Float|Ceil _returnvalue_4))
  (bind _returnvalue_6 (Math|Conversions|ToFloat(Integer) _returnvalue_5))
  (bind (_remainder _returnvalue_7) (Math|Float|Division(WholeandRemainder) _returnvalue_3 _returnvalue_6))
  ;[1 1 1] Clear Array
  (Utilities|Array|Clear (Variables|GridFormation|GetNewUnitPos))
  (Utilities|Array|Resize _rowarray _returnvalue_7)
  (Utilities|Array|Resize _col_array _returnvalue_5)
  (for (_ _array_index) _rowarray
    (for (_ _array_index_2) _col_array
      (Utilities|Array|Add _newunitpos (Math|Vector|MakeVector (+ _x (Math|Conversions|ToFloat(Integer) (* _array_index_2 _unit_position_offset_2))) (+ (* _array_index _unit_position_offset_2) _y) _z)))
    (Utilities|Array|Resize _remainderarray (Math|Float|Ceil _remainder))
    (for (_ _array_index_3) _remainderarray
      (Utilities|Array|Add (Variables|GridFormation|GetNewUnitPos) (Math|Vector|MakeVector (+ _x (* _array_index_3 _unit_position_offset)) (+ _y (* _returnvalue_7 _unit_position_offset)) _z))))
  (return _newunitpos))

(fn IsUnitsSelection
  (return (Utilities|Array|IsNotEmpty (Variables|Selection|GetUnitSelection))))

(fn ChangeCursor
  (params (Hover%20cursor%20hit :type Actor%20Object%20Reference))
  ;[1 1 1] Combat cursor
  (if (Utilities|ClassIsChildOf (Utilities|GetClass Hover%20cursor%20hit) "/Game/Actors/Combat/Group/Unit_EnemyKnight.Unit_EnemyKnight_C")
    (Variables|Default|SetCurrentMouseCursor "Crosshairs")
    (Variables|Default|SetIsHoverEnemy true)
    (Variables|Default|SetEnemyToAttack Hover%20cursor%20hit)
    (else
      (Variables|Default|SetCurrentMouseCursor "Default")
      (Variables|Default|SetIsHoverEnemy false))))

(fn GetEnemyPos
  (return (Transformation|GetActorLocation (Variables|Default|GetEnemyToAttack))))

(fn GetAllEnemies
  (bind _outactors (Actor|GetAllActorsOfClass "/Game/Actors/Combat/Group/Unit_EnemyKnight.Unit_EnemyKnight_C"))
  (return _outactors))

(fn BuildingPreview
  (bind _hitresult (Game|Player|GetHitResultUnderCursorbyChannel "TraceTypeQuery5" false))
  (Variables|Buildings|SetPlacementLoacation (Math|Conversions|ToTransform(Vector) (.location _hitresult)))
  (Transformation|SetActorLocation (Variables|Buildings|GetSelectedBuildingObj) (.location _hitresult) false false)
  (return))

(fn PlaceBuilding
  (for (_array_element _array_index) (Variables|Buildings|GetOriginalMaterials)
    (Rendering|Material|SetMaterial (Variables|Buildings|GetBuilding%20Mesh) _array_index _array_element)))

(fn RotateBuilding
  (params (NewParam :type Boolean))
  (bind (_deltax _deltay) (Class|PlayerController|GetInputMouseDelta))
  (bind _hitresult (Game|Player|GetHitResultUnderCursorbyChannel "TraceTypeQuery5" true))
  (bind _selectedbuildingobj (Variables|Buildings|GetSelectedBuildingObj))
  (bind _returnvalue (Transformation|GetActorLocation _selectedbuildingobj))
  (bind _returnvalue_2 (Math|Rotator|FindLookatRotation _returnvalue (.impactpoint _hitresult)))
  (if (> (Math|Vector|Distance(Vector) _returnvalue (.impactpoint _hitresult)) 1e+02)
    (if (> _deltax 0.0)
      (Audio|PlaySound2D "/Game/SoundEffects/UI/rotate.rotate" 1.0 1.0 0.0 "/Game/SoundEffects/UI/Soncur_Rotate.Soncur_Rotate" 0 :!label _label)
      (elif (< _deltay 0.0)
        (goto _label)
        (else
          _)))
    (Transformation|SetActorRotation (Variables|Buildings|GetSelectedBuildingObj) (Math|Rotator|MakeRotator 0.0 0.0 (.yaw _returnvalue_2)))
    (Variables|Buildings|SetRotationForRaycast (Math|Rotator|MakeRotator 0.0 0.0 (.yaw _returnvalue_2)))))

(fn EnemyOffset
  (params (Index :type Integer) (Enemy%20pos :type Vector))
  (bind _returnvalue (Math|Conversions|ToFloat(Integer) Index))
  (bind _unitselection (Variables|Selection|GetUnitSelection))
  (bind _returnvalue_2 (Utilities|Array|Length _unitselection))
  (bind _returnvalue_3 (Math|Conversions|ToFloat(Integer) _returnvalue_2))
  (bind _returnvalue_4 (/ _returnvalue _returnvalue_3))
  (bind _returnvalue_5 (* _returnvalue_4 3.6e+02))
  (return (+ Enemy%20pos (Math|Vector|MakeVector (Math|Trig|Cos(Degrees) _returnvalue_5) (Math|Trig|Sin(Degrees) _returnvalue_5) 0.0))))

(fn NotEnoughResources
  (Variables|Buildings|SetIsBuilding true))

(fn CancelBuilding
  (Actor|DestroyActor (Variables|Default|GetBuildingTarget))
  (Variables|Buildings|SetIsBuilding false)
  (Variables|Buildings|SetisRotatingBuilding false))

(fn BuildingPopUp
  (bind _returnvalue (Game|GetPlayerController 0))
  (bind (_locationx _locationy) (Game|Player|GetMousePosition _returnvalue))
  ;[1 1 1] check that hit is a building
  (if (Utilities|ClassIsChildOf (Utilities|GetClass (Variables|Default|GetHover%20Cursor%20Hit)) "/Game/Actors/Buildings/Blueprints/BP_BuildingBase.BP_BuildingBase_C")
    ;[1 1 1] add popup menu widget to viewport
    (bind _returnvalue_2 (UserInterface|CreateWidget "/Game/WBP_BuildingPopup.WBP_BuildingPopup_C"))
    (Variables|Default|SetBuildingPopupWidget _returnvalue_2)
    (bind _asbp_building_base (Utilities|Casting|CastToBP_BuildingBase (Variables|Default|GetHover%20Cursor%20Hit)))
    (Default|SetCurrentSelect (Variables|Default|GetBuildingPopupWidget) _asbp_building_base)
    (UserInterface|Viewport|AddtoViewport (Variables|Default|GetBuildingPopupWidget) 0)
    (Variables|Default|SetIs%20Pop%20Up%20Open true)
    ;[1 1 1] set widget position to hit cursor
    (Class|UserWidget|SetPositioninViewport (Variables|Default|GetBuildingPopupWidget) (Math|Vector2D|MakeVector2D _locationx _locationy) true)))

(fn IsHoverBuilding
  (params (Hit%20Object :type Actor%20Object%20Reference))
  (bind _returnvalue (Utilities|GetClass Hit%20Object))
  (bind _returnvalue_2 (Utilities|ClassIsChildOf _returnvalue "/Game/Actors/Buildings/Blueprints/BP_BuildingBase.BP_BuildingBase_C"))
  (bind _output_get (Variables|Default|SetIs%20Hover%20Building _returnvalue_2))
  (return _returnvalue_2))

(fn GetBuildingMaterials
  (bind _buildingtarget (Variables|Default|GetBuildingTarget))
  (bind _buildingmesh (Variables|/Game/Actors/Buildings/Blueprints/BP_BuildingBase.BP_BuildingBase_C|GetBuildingMesh _buildingtarget))
  (for (_ _array_index) (Rendering|Material|GetMaterials _buildingmesh)
    (Rendering|Material|SetMaterial _buildingmesh _array_index "/Game/Actors/Buildings/M_BuildingPreviewError.M_BuildingPreviewError")))

(fn PlacementCheck
  (bind _frontleft (LocalVariables|GetFrontLeft))
  (bind _frontright (LocalVariables|GetFrontRight))
  (bind _backleft (LocalVariables|GetBackLeft))
  (bind _backright (LocalVariables|GetBackRight))
  (bind _origin (LocalVariables|GetOrigin))
  (|GettingBoxCornerVectors)
  (bind _outhit (Class|KismetSystemLibrary|LineTraceSinglebyProfile (Math|Vector|MakeVector (.x _frontleft) (.y _frontleft) (+ (.z _frontleft) 2e+02)) (Math|Vector|MakeVector (.x _frontleft) (.y _frontleft) (- (.z _frontleft) 1e+03)) "PlaceBuilding" false (Utilities|Array|MakeArray (Variables|Buildings|GetSelectedBuildingObj)) "ForOneFrame" true "(R=1.000000,G=0.000000,B=0.790184,A=1.000000)"))
  (bind _outhit_2 (Class|KismetSystemLibrary|LineTraceSinglebyProfile (Math|Vector|MakeVector (.x _frontright) (.y _frontright) (+ (.z _frontright) 2e+02)) (Math|Vector|MakeVector (.x _frontright) (.y _frontright) (- (.z _frontright) 1e+03)) "PlaceBuilding" false (Utilities|Array|MakeArray (Variables|Buildings|GetSelectedBuildingObj)) "ForOneFrame" true))
  (bind _outhit_3 (Class|KismetSystemLibrary|LineTraceSinglebyProfile (Math|Vector|MakeVector (.x _backleft) (.y _backleft) (+ (.z _backleft) 2e+02)) (Math|Vector|MakeVector (.x _backleft) (.y _backleft) (- (.z _backleft) 1e+03)) "PlaceBuilding" false (Utilities|Array|MakeArray (Variables|Buildings|GetSelectedBuildingObj)) "ForOneFrame" true "(R=0.023159,G=0.000000,B=1.000000,A=1.000000)"))
  (bind _outhit_4 (Class|KismetSystemLibrary|LineTraceSinglebyProfile (Math|Vector|MakeVector (.x _backright) (.y _backright) (+ (.z _backright) 2e+02)) (Math|Vector|MakeVector (.x _backright) (.y _backright) (- (.z _backright) 1e+03)) "PlaceBuilding" false (Utilities|Array|MakeArray (Variables|Buildings|GetSelectedBuildingObj)) "ForOneFrame" true "(R=1.000000,G=0.781128,B=0.000000,A=1.000000)"))
  (bind _outhit_5 (Class|KismetSystemLibrary|LineTraceSinglebyProfile (Math|Vector|MakeVector (.x _origin) (.y _origin) (+ (.z _origin) 2e+02)) (Math|Vector|MakeVector (.x _origin) (.y _origin) (- (.z _origin) 1e+03)) "PlaceBuilding" false (Utilities|Array|MakeArray (Variables|Buildings|GetSelectedBuildingObj)) "ForOneFrame" true))
  (return (Math|Boolean|ANDBoolean (== (Utilities|GetClass (.hitactor _outhit_3)) "/Script/Landscape.LandscapeStreamingProxy") (== (Utilities|GetClass (.hitactor _outhit_4)) "/Script/Landscape.LandscapeStreamingProxy") (== (Utilities|GetClass (.hitactor _outhit_2)) "/Script/Landscape.LandscapeStreamingProxy") (== (Utilities|GetClass (.hitactor _outhit)) "/Script/Landscape.LandscapeStreamingProxy") (== (Utilities|GetClass (.hitactor _outhit_5)) "/Script/Landscape.LandscapeStreamingProxy"))))

(fn RemovebuildingPopup
  (params (Is%20building%20hovering :type Boolean))
  (bind _buildingpopupwidget (Variables|Default|GetBuildingPopupWidget))
  (if (not Is%20building%20hovering)
    (if (Utilities|IsValid _buildingpopupwidget)
      (Widget|RemovefromParent _buildingpopupwidget)
      (Variables|Default|SetIs%20Pop%20Up%20Open false))))

(fn BuildingOverlapCheck)

(fn CombatMenu
  (bind _hud_in_game (Variables|Default|GetHud%20in%20Game))
  (bind _wbp_hud_combatmenu (Variables|/Game/Blueprints/HUD/WBP_HUD_InGame.WBP_HUD_InGame_C|GetWBP_HUD_CombatMenu _hud_in_game))
  ;[1 1 1] if units are selected
  (if (Utilities|IsValid _wbp_hud_combatmenu)
    (if (not (Utilities|Array|IsEmpty (Variables|Selection|GetUnitSelection)))
      ;[1 1 1] close building menu and open combat
      (Default|CloseBuildingMenu _hud_in_game)
      (Widget|SetVisibility _wbp_hud_combatmenu "Visible")
      (Default|UpdateSelectedUnits _wbp_hud_combatmenu)
      (else
        (Widget|SetVisibility _wbp_hud_combatmenu "Hidden")))))

(fn TutorialIncriment
  (params (Tutorial%20stage :type Integer) (done :type Boolean)))

(fn DebrisParticles
  (params (BuildingTarget :type BP%20Building%20Base%20Object%20Reference))
  (bind _buildingmesh (Variables|/Game/Actors/Buildings/Blueprints/BP_BuildingBase.BP_BuildingBase_C|GetBuildingMesh BuildingTarget))
  (bind (_min _max) (Components|StaticMesh|GetLocalBounds _buildingmesh))
  (bind _returnvalue (- _max _min))
  (bind _returnvalue_2 (/ _returnvalue "1000.000000,1000.000000,300.000000"))
  (bind (_x _y _z) (Math|Vector|BreakVector _returnvalue_2))
  (bind _output_get (Variables|Default|SetDebris_System "/Game/Particles/FXS_Debris_System.FXS_Debris_System"))
  (bind _returnvalue_3 (Niagara|SpawnSystematLocation _output_get (Transformation|GetActorLocation BuildingTarget) (Transformation|GetActorRotation BuildingTarget) _returnvalue_2 true false))
  (Class|NiagaraComponent|SetVariableInt _returnvalue_3 "ParticleCount" (Math|Float|Truncate (Math|Float|Clamp(Float) (* _x _y _z 116.0) 5e+01 1.5e+03)))
  (Components|Activation|SetActive _returnvalue_3 true false))