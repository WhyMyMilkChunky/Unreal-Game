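; Base actor for buildings, which load stats, costs and meshes from DT_Buildings by type and pick one of two mesh variants at random.
; Tick traces for landscape during placement, then runs a production timer that feeds resources to BP_ResourceManager once built.
; It also handles cost checks, a single tier upgrade, foliage removal on overlap, and damage leading to destruction with bounds-scaled debris particles.
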(event OnComponentBeginOverlap(FoliageCollider)
  (params (OverlappedComponent :type Primitive%20Component%20Object%20Reference) (OtherActor :type Actor%20Object%20Reference) (OtherComp :type Primitive%20Component%20Object%20Reference) (OtherBodyIndex :type Integer) (bFromSweep :type Boolean) (SweepResult :type Hit%20Result%20Structure%20%28by%20ref%29))
  (bind _asfoliage_instanced_static_mesh_component (Utilities|Casting|CastToFoliageInstancedStaticMeshComponent OtherComp))
  (CallFunction|RemoveFoliage _asfoliage_instanced_static_mesh_component OtherBodyIndex))

(event Custom|Building%20Destroy
  (bind _buildingmesh (Variables|Default|GetBuildingMesh))
  (bind _buildingmesh_2 (Variables|Default|GetBuildingMesh))
  (bind (_min _max) (Components|StaticMesh|GetLocalBounds _buildingmesh))
  (bind _returnvalue (- _max _min))
  (bind _returnvalue_2 (/ _returnvalue "1000.000000,1000.000000,300.000000"))
  (bind (_x _y _z) (Math|Vector|BreakVector _returnvalue_2))
  (bind _output_get (Variables|Default|SetDebrisSystem "/Game/Particles/FXS_Debris_System.FXS_Debris_System"))
  (bind _returnvalue_3 (Niagara|SpawnSystematLocation _output_get (Transformation|GetWorldLocation _buildingmesh) (Transformation|GetWorldRotation _buildingmesh) _returnvalue_2 true false))
  (Class|NiagaraComponent|SetVariableInt _returnvalue_3 "ParticleCount" (Math|Float|Truncate (Math|Float|Clamp(Float) (* _x _y _z 116.0) 5e+01 1.5e+03)))
  (Components|Activation|SetActive _returnvalue_3 true false)
  (Rendering|SetVisibility _buildingmesh_2 false true)
  (Collision|SetCollisionEnabled _buildingmesh_2 "NoCollision")
  ;[1 1 1] Increased Delay For Particles, Disabled Collision to Midigate Interference
  (Utilities|FlowControl|Delay 2.0)
  (Actor|DestroyActor))

(event EventBeginPlay
  (bind _output_get (Variables|Default|SetBuildingName (Utilities|String|StringToName (Utilities|String|EnumtoString (Variables|Default|GetBuildingType)))))
  (bind (_buildingcategory _buildingtype _health _meshline1 _meshline2) (CallFunction|BuildingInit _output_get))
  (CallFunction|SetMesh _meshline1 (Variables|Default|GetUpgrade%20Tier) _meshline2)
  (bind _returnvalue (Actor|GetActorOfClass "/Game/Blueprints/Resources/BP_ResourceManager.BP_ResourceManager_C"))
  (Variables|Default|SetResourceManager _returnvalue)
  (Collision|SetCollisionEnabled (Variables|Default|GetBuildingMesh) "QueryAndPhysics"))

(event Collision|EventActorBeginOverlap
  (params (OtherActor :type Actor%20Object%20Reference)))

(event EventTick
  (params (DeltaSeconds :type Float%20%28single-precision%29))
  ;[1 1 1] actor placed
  (if (Utilities|Enum|Equal(Enum) (Variables|Default|GetBuilding%20Status) "NewEnumerator0")
    (CallFunction|CheckGround)
    (else
      ;[1 1 1] after being built
      (if (Utilities|Enum|Equal(Enum) (Variables|Default|GetBuilding%20Status) "NewEnumerator1")
        (CallFunction|FunctionDoTick)))))

(fn ConstructionScript
  (Collision|SetCollisionEnabled (Variables|Default|GetFoliageCollider) "NoCollision")
  (Collision|SetCollisionEnabled (Variables|Default|GetBuildingMesh) "NoCollision"))

(fn BuildingInit
  (params (BuildingName :type Name))
  (bind _returnvalue (Utilities|GetDataTableRow "/Game/Actors/Buildings/DT_Buildings.DT_Buildings" BuildingName)
    (:then
      (Variables|Default|SetBuildingData (Utilities|Struct|MakeF_BuildingStruct (.buildingcategory _returnvalue) (.buildingtype _returnvalue) (.startingmaxhealth _returnvalue) (.var1meshes _returnvalue) (.var2meshes _returnvalue) (.buildingcost _returnvalue) (.upgradecost _returnvalue) (.description _returnvalue) (.t1produce _returnvalue) (.t2produce _returnvalue) (.startingtotalsecondtoproduce _returnvalue) (.blueprintclass _returnvalue)))
      (Variables|Default|SetHealth (.startingmaxhealth _returnvalue)))
    (:RowNotFound
      _))
  (return (.buildingcategory _returnvalue) (.buildingtype _returnvalue) (.startingmaxhealth _returnvalue) (.var1meshes _returnvalue) (.var2meshes _returnvalue) (.buildingcost _returnvalue)))

(fn SetMesh
  (params (Array :type Array%20of%20Static%20Mesh%20Object%20References) (UpgradeTeir :type Integer) (Array2 :type Array%20of%20Static%20Mesh%20Object%20References))
  (bind _buildingmesh (Variables|Default|GetBuildingMesh))
  (switch int (Math|Random|RandomInteger 2)
    (:0
      (Components|StaticMesh|SetStaticMesh _buildingmesh (Utilities|Array|Get(acopy) Array UpgradeTeir)))
    (:1
      (Components|StaticMesh|SetStaticMesh _buildingmesh (Utilities|Array|Get(acopy) Array2 UpgradeTeir)))))

(fn BuildingCost
  ;[1 1 1] Use up the resources cost for building
  (for _array_element (.buildingcost (Variables|Default|GetBuildingData))
    (Default|SubtractResouce (Variables|Default|GetResourceManager) (.Resource (Utilities|Struct|BreakF_BuildingCosts _array_element)) (.Amount (Utilities|Struct|BreakF_BuildingCosts _array_element)))))

(fn CheckBuildingcost
  (bind _buildingdata (Variables|Default|GetBuildingData))
  (Utilities|Array|Clear (LocalVariables|Getbool%20check%20resources))
  (for _array_element (.buildingcost _buildingdata)
    (bind _quantity (Default|GetResource (Variables|Default|GetResourceManager) (.Resource (Utilities|Struct|BreakF_BuildingCosts _array_element))))
    (Utilities|Array|AddUnique (LocalVariables|Getbool%20check%20resources) (>= _quantity (.Amount (Utilities|Struct|BreakF_BuildingCosts _array_element)))))
  (Utilities|Array|Clear (LocalVariables|Getbool%20check%20upgrade))
  (for _array_element_2 (.upgradecost _buildingdata)
    (bind _quantity_2 (Default|GetResource (Variables|Default|GetResourceManager) (.Resource (Utilities|Struct|BreakF_BuildingCosts _array_element_2))))
    (Utilities|Array|AddUnique (LocalVariables|Getbool%20check%20upgrade) (>= _quantity_2 (.Amount (Utilities|Struct|BreakF_BuildingCosts _array_element_2)))))
  (return (not (Utilities|Array|ContainsItem (LocalVariables|Getbool%20check%20resources) false)) (not (Utilities|Array|ContainsItem (LocalVariables|Getbool%20check%20upgrade) false))))

(fn RemoveFoliage
  (params (InstancedComponent :type Foliage%20Instanced%20Static%20Mesh%20Component%20Object%20Reference) (Index :type Integer))
  (Class|InstancedStaticMeshComponent|RemoveInstance InstancedComponent Index))

(fn EnableFoliageRemoval
  (Collision|SetCollisionEnabled (Variables|Default|GetFoliageCollider) "QueryOnly"))

(fn CanbePlaced
  (params (Can%20Be%20Placed :type Boolean))
  (return Can%20Be%20Placed))

(fn IfResourceTimeReached
  ;[1 1 1] my if statement is better than your if statement
  (if (>= (Variables|Default|Getglobal%20current) (.startingtotalsecondtoproduce (Variables|Default|GetBuildingData)))
    (Variables|Default|Setglobal%20current 0.0)
    (CallFunction|DoFunction))
  (return))

(fn CalculateTimetoAddResource
  (params (Delta%20Time :type Float%20%28double-precision%29))
  ;[1 1 1] Timer (Cover For Regan)
  (Variables|Default|Setglobal%20current (+ (Variables|Default|Getglobal%20current) Delta%20Time))
  (return (/ (Variables|Default|Getglobal%20current) (.startingtotalsecondtoproduce (Variables|Default|GetBuildingData)))))

(fn SetBuildingCollision
  (Collision|SetCollisionEnabled (Variables|Default|GetBuildingMesh) "QueryAndPhysics"))

(fn DoFunction
  (bind _buildingdata (Variables|Default|GetBuildingData))
  (bind _keys (Utilities|Map|Keys (.t1produce _buildingdata)))
  (for _array_element _keys
    (Default|AddResource (Variables|Default|GetResourceManager) (.Value (Utilities|Map|Find (.t1produce _buildingdata) _array_element)) _array_element))
  (bind _asin_game_mode (Utilities|Casting|CastToInGameMode (Game|GetGameMode)))
  (Default|UpdateResourceUI _asin_game_mode))

(fn FunctionDoTick
  ;[1 1 1] calculate time and then do the function
  (CallFunction|IfResourceTimeReached)
  (bind _percent (CallFunction|CalculateTimetoAddResource (Utilities|Time|GetWorldDeltaSeconds)))
  (Variables|Default|SetPercentToProduce _percent))

(fn UpgradeBuilding
  (params (FromLoad? :type Boolean))
  (bind _buildingdata (Variables|Default|GetBuildingData))
  (if (== (Variables|Default|GetUpgrade%20Tier) 0)
    ;[1 1 1] Prevents Check for buildings on load
    (if FromLoad?
      (bind _result (Math|Integer|IncrementInt (Variables|Default|GetUpgrade%20Tier) :!label _label)
        (:%20%20
          (CallFunction|SetMesh (.var1meshes _buildingdata) _result (.var2meshes _buildingdata))
          ;[1 1 1] Prevents building sound on load
          (if (not FromLoad?)
            (Audio|PlaySound2D "/Game/SoundEffects/UI/BuildingBuild.BuildingBuild" 1.0 1.0 0.0 0 0))))
      (else
        (bind _hasenoughupgrade (CallFunction|CheckBuildingcost))
        (if _hasenoughupgrade
          (goto _label)
          (else
            (Audio|PlaySound2D "/Game/SoundEffects/VoiceLines/Not_Enough_Resources.Not_Enough_Resources" 1.0 1.0 0.0 0 0)
            (Audio|PlaySound2D "/Game/SoundEffects/UI/Error.Error" 1.0 1.0 0.0 0 0)))))))

(fn CheckGround
  (bind _returnvalue (Transformation|GetActorLocation))
  (bind _outhit (Class|KismetSystemLibrary|LineTraceSinglebyProfile (Math|Vector|MakeVector (.x _returnvalue) (.y _returnvalue) (+ (.z _returnvalue) 1e+02)) (Math|Vector|MakeVector (.x _returnvalue) (.y _returnvalue) (- (.z _returnvalue) 1e+02)) "BlockAll" false 0 "None" true))
  (CallFunction|CanbePlaced (== (Utilities|GetClass (.hitactor _outhit)) "/Script/Landscape.LandscapeStreamingProxy")))

(fn TakingDamage
  (bind _output_get (Variables|Default|SetHealth (- (Variables|Default|GetHealth) (Variables|Default|GetDamage))))
  (Development|PrintString (Utilities|String|ToString(Integer) _output_get))
  (if (<= _output_get 0)
    (Development|PrintString (Utilities|String|ToString(Integer) _output_get))
    (CallFunction|BuildingDestroy)))

(fn CheckResourceforProduction
  (params (Resource :type E_ResourceType%20Enum :default "NewEnumerator0") (Required%20resource%20quantity :type Integer))
  (return (<= Required%20resource%20quantity (.Value (Utilities|Map|Find (Variables|/Game/Blueprints/Resources/BP_ResourceManager.BP_ResourceManager_C|GetResources%20Map (Variables|Default|GetResourceManager)) Resource)))))