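; Butcher building that converts one input resource into produced resources through its Do Function.
; The upgrade tier selects the intake amount, which must pass a resource check before production runs.
; For each T1Produce entry in BuildingData, ResourceManager subtracts the intake and adds that output, then InGameMode refreshes the resource UI.
; Both tiers share the T1 output table, and the intake is charged once per output type.
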(event EventBeginPlay
  (|CallParentFunction) ; This node is disabled and will not be called.\nDrag off pins to build functionality.
)

(event Collision|EventActorBeginOverlap
  (params (OtherActor :type Actor%20Object%20Reference))
  (|CallParentFunction OtherActor) ; This node is disabled and will not be called.\nDrag off pins to build functionality.
)

(event EventTick
  (params (DeltaSeconds :type Float%20%28single-precision%29))
  (|CallParentFunction DeltaSeconds) ; This node is disabled and will not be called.\nDrag off pins to build functionality.
)

(fn ConstructionScript
  (|CallParentFunction))

(fn DoFunction
  (bind _buildingdata (Variables|Default|GetBuildingData))
  (bind _resourcemanager (Variables|Default|GetResourceManager))
  ;[1 1 1] check resource intake by upgrade tier
  (switch int (Variables|Default|GetUpgrade%20Tier)
    (:Default
      (bind _output_get (LocalVariables|SetResource%20intake (Variables|Default|GetResource%20intake%20T1) :!label _label))
      ;[1 1 1] check if their is enough of the resource intake
      (bind _has_enough_resource (CallFunction|CheckResourceforProduction "NewEnumerator11" _output_get))
      (if _has_enough_resource
        (bind _keys (Utilities|Map|Keys (.t1produce _buildingdata) :!label _label_2))
        (for _array_element _keys
          (Default|SubtractResouce _resourcemanager "NewEnumerator11" (LocalVariables|GetResource%20intake))
          (Default|AddResource _resourcemanager (.Value (Utilities|Map|Find (.t1produce _buildingdata) _array_element)) _array_element))
        (bind _asin_game_mode (Utilities|Casting|CastToInGameMode (Game|GetGameMode)))
        (Default|UpdateResourceUI _asin_game_mode)))
    (:0
      (goto _label))
    (:1
      (bind _output_get_2 (LocalVariables|SetResource%20intake (Variables|Default|Getresource%20intake%20t2)))
      (bind _has_enough_resource_2 (CallFunction|CheckResourceforProduction "NewEnumerator11" _output_get_2))
      (if _has_enough_resource_2
        (goto _label_2)))))