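; Mine building actor that produces resources for the player when its Do Function runs.
; It reads the tier 1 or tier 2 produce map from its building data depending on UpgradeTier, then adds each resource and amount through the ResourceManager.
; Afterwards it tells the InGameMode game mode to refresh the resource UI.
; The event graph and construction script add no logic of their own.
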(event EventBeginPlay
  (|CallParentFunction) ; This node is disabled and will not be called.\nDrag off pins to build functionality.
)

(event Collision|EventActorBeginOverlap
  (params (OtherActor :type Actor%20Object%20Reference))
  (|CallParentFunction OtherActor) ; This node is disabled and will not be called.\nDrag off pins to build functionality.
)

(event EventTick
  (params (DeltaSeconds :type Float%20%28single-precision%29))
  (|CallParentFunction DeltaSeconds) ; This node is disabled and will not be called.\nDrag off pins to build functionality.
)

(fn ConstructionScript
  (|CallParentFunction))

(fn DoFunction
  (bind _buildingdata (Variables|Default|GetBuildingData))
  (bind _resourcemanager (Variables|Default|GetResourceManager))
  (if (== (Variables|Default|GetUpgrade%20Tier) 0)
    (bind _keys (Utilities|Map|Keys (.t1produce _buildingdata)))
    (for _array_element _keys
      (Default|AddResource _resourcemanager (.Value (Utilities|Map|Find (.t1produce _buildingdata) _array_element)) _array_element))
    (else
      (bind _keys_2 (Utilities|Map|Keys (.t2produce _buildingdata)))
      (for _array_element_2 _keys_2
        (Default|AddResource _resourcemanager (.Value (Utilities|Map|Find (.t2produce _buildingdata) _array_element_2)) _array_element_2))))
  (bind _asin_game_mode (Utilities|Casting|CastToInGameMode (Game|GetGameMode)))
  (Default|UpdateResourceUI _asin_game_mode))