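; BP_Banner is a banner actor that spawns with a small debris effect and turns to face the player.
; BeginPlay activates a tiny-scaled debris particle system at the actor and drops the banner mesh below its placed height.
; Tick billboards the banner on yaw toward the first player's camera, then after a one-tick delay plays a Timeline that increments its Z, gated by a comparison with BannerZValue.
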(event EventBeginPlay
  (bind _banner (Variables|Default|GetBanner))
  (bind _returnvalue (Transformation|GetWorldLocation _banner))
  (Utilities|FlowControl|Sequence
    (:then_0
      ;[1 1 1] particles
      (bind _returnvalue_2 (Niagara|SpawnSystematLocation "/Game/Particles/FXS_Debris_System.FXS_Debris_System" (Transformation|GetActorLocation) "0, 0, 0" "0.001000,0.001000,0.001000" true false))
      (Class|NiagaraComponent|SetVariableInt _returnvalue_2 "ParticleCount" (Math|Float|Truncate 5.0))
      (Components|Activation|SetActive _returnvalue_2 true false)
      ;[1 1 1] set below map
      (Transformation|SetWorldLocation _banner (Math|Vector|MakeVector (.x _returnvalue) (.y _returnvalue) (- (.z _returnvalue) 5e+01)) false false))))

(event Collision|EventActorBeginOverlap
  (params (OtherActor :type Actor%20Object%20Reference)))

(event EventTick
  (params (DeltaSeconds :type Float%20%28single-precision%29))
  (bind _banner (Variables|Default|GetBanner))
  (bind _returnvalue (Transformation|GetWorldLocation _banner))
  (CallFunction|BilboardBanner)
  (Utilities|FlowControl|DelayUntilNextTick)
  (Timeline|Timeline Play
    (:Update
      ;[1 1 1] get world pos of banner and lower it to start
      (if (not (< (.z (Transformation|GetWorldLocation (Variables|Default|GetBanner))) (Variables|Default|GetBanner%20Z%20value)))
        ;[1 1 1] set its position with incremented Z
        (bind _result (Math|Float|IncrementFloat (.z (Transformation|GetWorldLocation (Variables|Default|GetBanner))))
          (:%20%20
            (Transformation|SetWorldLocation _banner (Math|Vector|MakeVector (.x _returnvalue) (.y _returnvalue) _result) false false)))))))

(fn ConstructionScript)

(fn BilboardBanner
  (Transformation|SetWorldRotation (Variables|Default|GetBanner) (Math|Rotator|MakeRotator 0.0 0.0 (.Yaw (Math|Rotator|BreakRotator (Math|Rotator|FindLookatRotation (Transformation|GetWorldLocation (Variables|Default|GetBanner)) (Camera|GetCameraLocation (Variables|/Script/Engine.PlayerController|GetPlayerCameraManager (Game|GetPlayerController 0))))))) false false))