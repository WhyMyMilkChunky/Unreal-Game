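; Base RTS combat unit for both sides, holding stats and handling click selection through BP_PlayerController with a decal.
; Tick checks health, destroys dead units after removing them from opponents' arrays, and steers enemies to the nearest Friendly-tagged actor or player building.
; Movement uses AIMoveTo or a blackboard TargetLocation.
; Opponent lists cover only knight classes, and the damage-dealing attack event is called only from disconnected in-range logic.
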(event Custom|isSelected
  (params (isSelected :type Boolean))
  (bind _decal (Variables|Default|GetDecal))
  ;[1 1 1] Unit Selection
  (Rendering|SetVisibility (Variables|Default|GetDecal) isSelected false)
  (Rendering|Components|Decal|SetFadeOut _decal 0.0 0.0 true)
  (Rendering|Components|Decal|SetFadeScreenSize _decal 0.0))

(event Custom|IfEnemyInRange
  (params (Unit :type BP%20Unit%20Base%20Object%20Reference) (Enemy :type BP%20Unit%20Base%20Object%20Reference))
  ;[1 1 1] Attack
  (Utilities|FlowControl|Delay (.attackspeed (Variables|Type|GetUnitStats)))
  (CallFunction|Attacking Unit Enemy)
  (Development|PrintString (Utilities|String|Append (Utilities|GetDisplayName self) "  is attacking: " (Utilities|GetDisplayName Enemy))))

(event Custom|Die
  ;[1 1 1] Die Event
  ;[1 1 1] delete self from other units arrays
  (Variables|UnitStats|SetIsDead true)
  (for _array_element (Variables|Default|GetAll%20Enemys)
    (if (Utilities|Array|IsValidIndex (Variables|BP_UnitBase_C|GetAll%20Enemys _array_element) (Utilities|Array|FindItem (Variables|BP_UnitBase_C|GetAll%20Enemys _array_element) self))
      (Utilities|Array|RemoveIndex (Variables|BP_UnitBase_C|GetAll%20Enemys _array_element) (Utilities|Array|FindItem (Variables|BP_UnitBase_C|GetAll%20Enemys _array_element) self))
      (CallFunction|UpdateArray)))
  (Actor|DestroyActor))

(event EventBeginPlay
  (bind _asbp_player_controller (Utilities|Casting|CastToBP_PlayerController (Game|GetPlayerController 0)))
  (Variables|Default|SetAs%20BP%20Player%20Controller _asbp_player_controller)
  (CallFunction|UpdateArray)
  (Combat|GetAllPossibleTargets))

(event MouseInput|EventActorOnClicked
  (params (ButtonPressed :type Key%20Structure))
  ;[1 1 1] Unit Selection
  (if (and (== ButtonPressed "LeftMouseButton") (not (Variables|Type|GetIsEnemy)))
    (bind _asbp_player_controller (Utilities|Casting|CastToBP_PlayerController (Game|GetPlayerController 0)))
    (Variables|Default|SetAs%20BP%20Player%20Controller _asbp_player_controller)
    (if (Rendering|IsVisible (Variables|Default|GetDecal))
      (Default|RemoveUnitfromSelection (Variables|Default|GetAs%20BP%20Player%20Controller) self)
      (else
        (Default|AddUnittoSelectiom (Variables|Default|GetAs%20BP%20Player%20Controller) self)))))

(event EventTick
  (params (DeltaSeconds :type Float%20%28single-precision%29))
  ;[1 1 1] Check if Self is dead First
  (Class|AnimationBudgetBlueprintLibrary|EnableAnimationBudget false)
  (bind _isdead (CallFunction|CalculateDeath self))
  (if _isdead
    (CallFunction|Die))
  ;[1 0.4583 0.4583] If Enemy change behaviour
  (if (Variables|Type|GetIsEnemy)
    (switch Utilities|FlowControl|Switch|SwitchonE_EnemyBehaviors (Variables|Default|GetEnemy%20Behaviors)
      (:NewEnumerator0
        (bind _possible_targets (Combat|GetAllPossibleTargets))
        (bind _closest_target (Combat|GetClosestTarget _possible_targets))
        (AI|AIMoveTo self "0, 0, 0" _closest_target 5e+01 false))
      (:NewEnumerator1
        (Combat|AttackNearestBuilding)))))

(fn ConstructionScript)

(fn GotoEnemy
  (params (Enemy%20Location :type Vector)))

(fn Attacking
  (params (EnemyAttacking :type BP%20Unit%20Base%20Object%20Reference))
  (Variables|BP_UnitBase_C|SetUnitStats EnemyAttacking (Utilities|Struct|MakeF_UnitStats (.movementspeed (Variables|BP_UnitBase_C|GetUnitStats EnemyAttacking)) (.attackspeed (Variables|BP_UnitBase_C|GetUnitStats EnemyAttacking)) (.damage (Variables|BP_UnitBase_C|GetUnitStats EnemyAttacking)) (.soldiertype (Variables|BP_UnitBase_C|GetUnitStats EnemyAttacking)) (- (.health (Variables|BP_UnitBase_C|GetUnitStats EnemyAttacking)) (.damage (Variables|Type|GetUnitStats))) 0)))

(fn GetEnemyDistance
  (params (Enemy%20Unit :type BP%20Unit%20Base%20Object%20Reference))
  ;[1 1 1] if enemy is not dead and is in range INTERESTING
  (return (and (not (Variables|BP_UnitBase_C|GetIsDead Enemy%20Unit)) (<= (Math|Vector|Distance(Vector) (Transformation|GetActorLocation) (Transformation|GetActorLocation Enemy%20Unit)) 0.0))))

(fn CalculateDeath
  (params (Bp%20Unit :type BP%20Unit%20Base%20Object%20Reference))
  (return (and (<= (.health (Variables|Type|GetUnitStats)) 0.0) (not (Variables|BP_UnitBase_C|GetIsDead Bp%20Unit)))))

(fn UpdateArray
  (Utilities|Array|Clear (Variables|Default|GetAll%20Enemys))
  ;[1 1 1] only gets knights right now
  (bind _unit_array (CallFunction|GetAnyUnitArray (not (Variables|Type|GetIsEnemy)) "NewEnumerator0"))
  (Variables|Default|SetAll%20Enemys _unit_array))

(fn GetAnyUnitArray
  (params (isEnemy :type Boolean) (SoldierType :type SoldierTypes%20Enum :default "NewEnumerator0"))
  (if isEnemy
    (switch Utilities|FlowControl|Switch|SwitchonSoldierTypes SoldierType
      (:NewEnumerator0
        ;[1 1 1] sorry if theres a better way i made this at 5am
        (bind _outactors (Actor|GetAllActorsOfClass "/Game/Actors/Combat/Group/Unit_EnemyKnight.Unit_EnemyKnight_C"))
        (for _array_element _outactors
          (if (not (== (Variables|Type|GetIsEnemy self) (Variables|BP_UnitBase_C|GetIsEnemy _array_element)))
            (if (not (Variables|BP_UnitBase_C|GetIsDead _array_element))
              (Utilities|Array|Add (LocalVariables|GetUnitArray) _array_element)
              (for _array_element_2 (LocalVariables|GetUnitArray)
                _)
              (return (LocalVariables|GetUnitArray))))))
      (:NewEnumerator1
        (bind _outactors_2 (Actor|GetAllActorsOfClass "/Game/Actors/Combat/Group/Unit_EnemyKnight.Unit_EnemyKnight_C"))
        (for _array_element_3 _outactors_2
          (if (not (== (Variables|Type|GetIsEnemy self) (Variables|BP_UnitBase_C|GetIsEnemy _array_element_3)))
            (if (not (Variables|BP_UnitBase_C|GetIsDead _array_element_3))
              (Utilities|Array|Add (LocalVariables|GetUnitArray) _array_element_3)
              (for _array_element_4 (LocalVariables|GetUnitArray)
                _)
              (return (LocalVariables|GetUnitArray))))))
      (:NewEnumerator2
        (bind _outactors_3 (Actor|GetAllActorsOfClass "/Game/Actors/Combat/Group/Unit_EnemyKnight.Unit_EnemyKnight_C"))
        (for _array_element_5 _outactors_3
          (if (not (== (Variables|Type|GetIsEnemy self) (Variables|BP_UnitBase_C|GetIsEnemy _array_element_5)))
            (if (not (Variables|BP_UnitBase_C|GetIsDead _array_element_5))
              (Utilities|Array|Add (LocalVariables|GetUnitArray) _array_element_5)
              (for _array_element_6 (LocalVariables|GetUnitArray)
                _)
              (return (LocalVariables|GetUnitArray)))))))
    (else
      (switch Utilities|FlowControl|Switch|SwitchonSoldierTypes SoldierType
        (:NewEnumerator0
          (bind _outactors_4 (Actor|GetAllActorsOfClass "/Game/Actors/Combat/Group/Unit_Knight.Unit_Knight_C"))
          (for _array_element_7 _outactors_4
            (if (not (== (Variables|Type|GetIsEnemy self) (Variables|BP_UnitBase_C|GetIsEnemy _array_element_7)))
              (if (not (Variables|BP_UnitBase_C|GetIsDead _array_element_7))
                (Utilities|Array|Add (LocalVariables|GetUnitArray) _array_element_7)
                (for (_array_element_8 _array_index) (LocalVariables|GetUnitArray)
                  _)
                (return (LocalVariables|GetUnitArray))))))
        (:NewEnumerator1
          (bind _outactors_5 (Actor|GetAllActorsOfClass "/Game/Actors/Combat/Group/Unit_Knight.Unit_Knight_C"))
          (for _array_element_9 _outactors_5
            (if (not (== (Variables|Type|GetIsEnemy self) (Variables|BP_UnitBase_C|GetIsEnemy _array_element_9)))
              (if (not (Variables|BP_UnitBase_C|GetIsDead _array_element_9))
                (Utilities|Array|Add (LocalVariables|GetUnitArray) _array_element_9)
                (for (_array_element_10 _array_index_2) (LocalVariables|GetUnitArray)
                  _)
                (return (LocalVariables|GetUnitArray))))))
        (:NewEnumerator2
          (bind _outactors_6 (Actor|GetAllActorsOfClass "/Game/Actors/Combat/Group/Unit_Knight.Unit_Knight_C"))
          (for _array_element_11 _outactors_6
            (if (not (== (Variables|Type|GetIsEnemy self) (Variables|BP_UnitBase_C|GetIsEnemy _array_element_11)))
              (if (not (Variables|BP_UnitBase_C|GetIsDead _array_element_11))
                (Utilities|Array|Add (LocalVariables|GetUnitArray) _array_element_11)
                (for (_array_element_12 _array_index_3) (LocalVariables|GetUnitArray)
                  _)
                (return (LocalVariables|GetUnitArray))))))))))

(fn IfRemovefromArray
  (params (ArrayEnemies :type Array%20of%20BP%20Unit%20Base%20Object%20References))
  (for (_array_element _array_index) ArrayEnemies
    (if (== (Variables|BP_UnitBase_C|GetIsEnemy _array_element) (Variables|Type|GetIsEnemy))
      (Utilities|Array|RemoveIndex ArrayEnemies _array_index)
      (return false))))

(fn CheckNearestBuilding
  (bind _distances (Variables|Default|GetDistances))
  (bind _player_buildings (Variables|Default|GetPlayer%20Buildings))
  (Utilities|Array|Clear (Variables|Default|GetDistances))
  (for _array_element _player_buildings
    (Utilities|Array|Add _distances (Math|Vector|VectorLength (- (Transformation|GetActorLocation _array_element) (Transformation|GetActorLocation)))))
  (return (Utilities|Array|Get(acopy) _player_buildings (.IndexOfMinValue (Math|Float|MinOfFloatArray _distances)))))

(fn MoveEnemytoNearestBuilding
  (params (Closest%20Building :type BP%20Building%20Base%20Object%20Reference))
  (AI|Components|Blackboard|SetValueasVector (AI|GetBlackboard 0) (Utilities|Name|MakeLiteralName "TargetLocation") (Transformation|GetActorLocation Closest%20Building)))

(fn GetAllPlayerBuildings
  (return 0))

(fn Moveto
  (params (Target%20Position :type Vector))
  (Components|Movement|StopMovementImmediately (Variables|Character|GetCharacterMovement))
  (AI|Components|Blackboard|SetValueasVector (AI|GetBlackboard 0) (Utilities|Name|MakeLiteralName "TargetLocation") Target%20Position))

(fn SetSelf
  (params (Is%20Enemy :type Boolean) (movementspeed :type Float%20%28double-precision%29) (Attack%20speed :type Float%20%28double-precision%29) (Damage :type Float%20%28double-precision%29) (Soldier%20Type :type SoldierTypes%20Enum :default "NewEnumerator0") (health :type Float%20%28double-precision%29))
  (bind _output_get (Variables|Type|SetUnitStats (Utilities|Struct|MakeF_UnitStats movementspeed Attack%20speed Damage Soldier%20Type health "/Game/HUD/UI_Sprites/T_Icon_Archer.T_Icon_Archer")))
  (Variables|UnitStats|SetIsDead false)
  (Variables|Type|SetIsEnemy Is%20Enemy)
  (Variables|/Script/Engine.CharacterMovementComponent|SetMaxAcceleration (Variables|Character|GetCharacterMovement) (.movementspeed _output_get)))

(fn GetAllPossibleTargets
  (bind _outactors (Actor|GetAllActorswithTag "Friendly"))
  (return _outactors))

(fn GetClosestTarget
  (params (PossibleTargets :type Array%20of%20Actor%20Object%20References))
  (bind _target_distances (LocalVariables|GetTarget%20Distances))
  (Utilities|Array|Clear _target_distances)
  (for _array_element PossibleTargets
    (Utilities|Array|Add (LocalVariables|GetTarget%20Distances) (Math|Vector|VectorLength (- (Transformation|GetActorLocation _array_element) (Transformation|GetActorLocation)))))
  (return (Utilities|Array|Get(acopy) PossibleTargets (.IndexOfMinValue (Math|Float|MinOfFloatArray _target_distances)))))

(fn AttackNearestBuilding
  (if (not (Utilities|Array|IsEmpty (Variables|Default|GetPlayer%20Buildings)))
    (bind _closestbuilding (CallFunction|CheckNearestBuilding))
    (CallFunction|MoveEnemytoNearestBuilding _closestbuilding)))