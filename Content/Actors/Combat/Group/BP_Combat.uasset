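; BP_Combat is a group combat Blueprint that wears down an enemy count over time, apparently as an unfinished prototype.
; Combat is flagged on at BeginPlay, and Tick feeds a Delay that throttles the math to about once per second.
; Each step subtracts outgoing damage from the enemy count, while friendly losses and debug prints are disconnected.
; A damage multiplier function only fetches data table row names and is never called here.
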(event Custom|Combat%20Timer
  (Utilities|FlowControl|Delay 1.0)
  (CallFunction|CombatMath))

(event EventBeginPlay
  (Variables|Math|SetDamageBase 1)
  (Variables|Math|SetisInCombat true))

(event EventTick
  (params (DeltaSeconds :type Float%20%28single-precision%29))
  (if (Variables|Math|GetisInCombat)
    (CallFunction|CombatTimer)))

(fn ConstructionScript)

(fn CombatMath
  ;[1 1 1] Display damage Debug
  (bind _output_get (Variables|Math|SetEnemyCount (- (Variables|Math|GetEnemyCount) (Variables|Math|GetDamageOutgoing)))))

(fn DamageMultiplier
  (DataTable|GetDataTableRowNames "/Game/Actors/Combat/Group/DamageMultipliers.DamageMultipliers"))