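; Base troop actor for combat units, taking its appearance from a Knight, Archer or Calvary unit type.
; The construction script picks the skeletal mesh per type, with only the Archer also assigned an animation Blueprint.
; BeginPlay enables animation budgeting, and Tick snaps height to a downward trace's impact point without checking for a hit.
; Under a Move command, Tick also steers toward MoveLocation via MoveUnitWithSteering and updates IsMoving.
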(event EventBeginPlay
  (Class|AnimationBudgetBlueprintLibrary|EnableAnimationBudget true))

(event Collision|EventActorBeginOverlap
  (params (OtherActor :type Actor%20Object%20Reference)))

(event EventTick
  (params (DeltaSeconds :type Float%20%28single-precision%29))
  (CallFunction|StayGrounded)
  (switch Utilities|FlowControl|Switch|SwitchonE_Command (Variables|Default|GetCurrent%20Command)
    (:NewEnumerator0
      (CallFunction|MoveLogic))))

(fn ConstructionScript
  (bind _skeletalmesh (Variables|Default|GetSkeletalMesh))
  (switch Utilities|FlowControl|Switch|SwitchonSoldierTypes (Variables|Default|GetUnit%20Type)
    (:NewEnumerator0
      (Components|SkeletalMesh|SetSkeletalMeshAsset _skeletalmesh "/Game/Characters/Mannequin_UE4/Meshes/SK_Mannequin.SK_Mannequin"))
    (:NewEnumerator1
      (Components|SkeletalMesh|SetSkeletalMeshAsset _skeletalmesh "/Game/Actors/Combat/Models/SM_Archer.SM_Archer")
      (Components|Animation|SetAnimationMode (Variables|Default|GetSkeletalMesh) "AnimationBlueprint" true)
      (Class|SkeletalMeshComponent|SetAnimClass (Variables|Default|GetSkeletalMesh) "/Game/Actors/Combat/Group/ABP_Archer.ABP_Archer_C"))
    (:NewEnumerator2
      (Components|SkeletalMesh|SetSkeletalMeshAsset _skeletalmesh "/Game/Characters/Mannequin_UE4/Meshes/SK_Mannequin.SK_Mannequin"))))

(fn MoveLogic
  (bind _move_location (Variables|Default|GetMove%20Location))
  (bind _returnvalue (Class|UnitBPFunctionLibrary|MoveUnitwithSteering self (Math|Vector|MakeVector (.x _move_location) (.y _move_location) (.z (Transformation|GetActorLocation))) (Utilities|Time|GetWorldDeltaSeconds) 6e+02 5.0 45.0 3e+02))
  (Variables|Default|SetIsMoving (not _returnvalue)))

(fn StayGrounded
  (bind _returnvalue (Transformation|GetActorLocation))
  (bind _outhit (Collision|LineTraceByChannel (Math|Vector|MakeVector (.x _returnvalue) (.y _returnvalue) (+ (.z _returnvalue) 1e+02)) (Math|Vector|MakeVector (.x _returnvalue) (.y _returnvalue) (+ (.z _returnvalue) -2e+02)) "TraceTypeQuery5" false 0 "ForOneFrame"))
  (Transformation|SetActorLocation (Math|Vector|MakeVector (.x _returnvalue) (.y _returnvalue) (.z (.impactpoint _outhit))) false false))