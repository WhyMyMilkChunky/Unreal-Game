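; Troop controller actor that spawns friendly troops and enemy waves and issues RTS-style orders to selected troops.
; BeginPlay spawns a row of friendly troops; pressing P spawns enemies set to attack random friendlies.
; Right-click cancels building placement, targets an enemy, or computes formation positions for a move.
; Tick pushes the current command to selected troops and reassigns targets from cached troop arrays.
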(event Custom|Spawn%20Enemy%20Wave
  (params (Troop%20Class :type BP%20Base%20Troop%20Class%20Reference))
  (for _index (range 0 6)
    ;[1 1 1] Hard spawning enemies nroth of starting village
    (bind _troop (CallFunction|SpawnTroop (Math|Vector|MakeVector (Math|Random|RandomFloatinRange 1.215e+04 1.275e+04) (Math|Float|Clamp(Float) (* _index (Math|Random|RandomFloatinRange 9.3e+02 2317.5)) 2e+03 13905.0) 3.2e+02) "NewEnumerator1" Troop%20Class))
    (Utilities|Array|Add (Variables|Default|GetEnemyTroops) _troop))
  (for _array_element (Variables|Default|GetEnemyTroops)
    (Variables|/Game/Actors/Combat/NewAI/BP_BaseTroop.BP_BaseTroop_C|SetCurrent%20Target _array_element (.OutItem (Utilities|Array|Random (Variables|Default|GetFriendlyTroops))))
    (Variables|/Game/Actors/Combat/NewAI/BP_BaseTroop.BP_BaseTroop_C|SetCurrent%20Command _array_element "NewEnumerator1")))

(event EventBeginPlay
  (for _index (range 0 16)
    (CallFunction|SpawnTroop (Math|Vector|MakeVector -1.95e+03 (Math|Conversions|ToFloat(Integer) (+ (* _index 100) 1930)) 0.0) "NewEnumerator1" "/Game/Actors/Combat/NewAI/BP_FriendlyTroop.BP_FriendlyTroop_C")
    (bind _asbp_player_controller (Utilities|Casting|CastToBP_PlayerController (Game|GetPlayerController 0)))
    (Variables|Default|SetAs%20Player%20Controller _asbp_player_controller))
  (bind _outactors (Actor|GetAllActorsOfClass "/Game/Actors/Combat/NewAI/BP_FriendlyTroop.BP_FriendlyTroop_C"))
  (Variables|Default|SetFriendlyTroops _outactors))

(event Collision|EventActorBeginOverlap
  (params (OtherActor :type Actor%20Object%20Reference)))

(event EventTick
  (params (DeltaSeconds :type Float%20%28single-precision%29))
  (bind _enemytroops (Variables|Default|GetEnemyTroops))
  (bind _selectedtroops (Variables|Default|GetSelectedTroops))
  (bind _friendlytroops (Variables|Default|GetFriendlyTroops))
  (bind _returnvalue (Utilities|Array|Length _enemytroops))
  (bind _returnvalue_2 (- _returnvalue 1))
  (bind _output (Utilities|Array|Get(acopy) _enemytroops _returnvalue_2))
  (Variables|Default|SetDelta%20Time DeltaSeconds)
  (Utilities|FlowControl|Sequence
    (:then_0
      (switch Utilities|FlowControl|Switch|SwitchonE_Command (Variables|Default|GetCommand)
        (:NewEnumerator0
          ;[1 1 1] Nigga
          (for (_array_element _array_index) (Variables|Default|GetSelectedTroops)
            (Variables|/Game/Actors/Combat/NewAI/BP_BaseTroop.BP_BaseTroop_C|SetCurrent%20Command _array_element "NewEnumerator0")
            (Variables|/Game/Actors/Combat/NewAI/BP_BaseTroop.BP_BaseTroop_C|SetMove%20Location _array_element (Math|Vector|MakeVector (.x (Utilities|Array|Get(acopy) (Variables|FormationLocations|GetFormationLocations) _array_index)) (.y (Utilities|Array|Get(acopy) (Variables|FormationLocations|GetFormationLocations) _array_index)) 0.0))))
        (:NewEnumerator1
          (for (_array_element_2 _array_index_2) _selectedtroops
            (if (Utilities|IsValid _array_element_2)
              (Variables|/Game/Actors/Combat/NewAI/BP_BaseTroop.BP_BaseTroop_C|SetCurrent%20Command _array_element_2 "NewEnumerator1")
              (bind _output_get (Variables|/Game/Actors/Combat/NewAI/BP_BaseTroop.BP_BaseTroop_C|SetCurrent%20Target _array_element_2 (Variables|Default|Gettarget)))
              (if (not (Utilities|IsValid _output_get))
                (if (Utilities|IsValid _output)
                  (Variables|/Game/Actors/Combat/NewAI/BP_BaseTroop.BP_BaseTroop_C|SetCurrent%20Target _array_element_2 _output)
                  (if (<= (Utilities|Array|Length (Variables|Default|GetEnemyTroops)) 0)
                    (for _array_element_3 (Variables|Default|GetSelectedTroops)
                      (Variables|/Game/Actors/Combat/NewAI/BP_BaseTroop.BP_BaseTroop_C|SetCurrent%20Command _array_element_3 "NewEnumerator2")
                      (Variables|/Game/Actors/Combat/NewAI/BP_BaseTroop.BP_BaseTroop_C|SetisAttacking _array_element_3 false)))))
              (else
                (Utilities|Array|RemoveIndex _selectedtroops _array_index_2)))))))
    (:then_1
      (for _array_element_4 (Variables|Default|GetEnemyTroops)
        (switch Utilities|FlowControl|Switch|SwitchonE_Command (Variables|/Game/Actors/Combat/NewAI/BP_BaseTroop.BP_BaseTroop_C|GetCurrent%20Command _array_element_4)
          (:NewEnumerator1
            (if (Utilities|IsValid _array_element_4)
              (if (!= (Variables|/Game/Actors/Combat/NewAI/BP_BaseTroop.BP_BaseTroop_C|GetCurrent%20Target _array_element_4) "/Game/Actors/Combat/NewAI/BP_FriendlyTroop.BP_FriendlyTroop")
                (Variables|/Game/Actors/Combat/NewAI/BP_BaseTroop.BP_BaseTroop_C|SetCurrent%20Target _array_element_4 (Utilities|Array|Get(acopy) _friendlytroops (- (Utilities|Array|Length _friendlytroops) 1)))
                (if (<= (Utilities|Array|Length (Variables|Default|GetFriendlyTroops)) 0)
                  (Variables|/Game/Actors/Combat/NewAI/BP_BaseTroop.BP_BaseTroop_C|SetCurrent%20Command _array_element_4 "NewEnumerator2")
                  (Variables|/Game/Actors/Combat/NewAI/BP_BaseTroop.BP_BaseTroop_C|SetisAttacking _array_element_4 false))))))))))

(event Input|MouseEvents|RightMouseButton
  (params (Key :type Key%20Structure :default "None"))
  (bind _returnvalue (Game|GetPlayerController 0))
  (bind _as_player_controller (Variables|Default|GetAs%20Player%20Controller))
  (bind _hitresult (Game|Player|GetHitResultUnderCursorbyChannel _returnvalue "TraceTypeQuery1" false))
  (:Pressed
    (if (or (Variables|/Game/Actors/Player/BP_PlayerController.BP_PlayerController_C|GetIsBuilding _as_player_controller) (Variables|/Game/Actors/Player/BP_PlayerController.BP_PlayerController_C|GetisRotatingBuilding _as_player_controller))
      (Default|CancelBuilding _as_player_controller)
      (elif (== (Utilities|GetClass (.hitactor _hitresult)) "/Game/Actors/Combat/NewAI/BP_EnemyTroop.BP_EnemyTroop_C")
        (Variables|Default|Settarget (.hitactor _hitresult))
        (Variables|Default|SetCommand "NewEnumerator1")
        (else
          (Variables|FormationLocations|SetHit%20Result%20Impact%20Point (.impactpoint (.HitResult (Game|Player|GetHitResultUnderCursorbyChannel (Game|GetPlayerController 0) "TraceTypeQuery5" true))))
          (Variables|Default|SetCommand "NewEnumerator0")
          (bind _returnvalue_2 (Class|UnitBPFunctionLibrary|GetFormationPositions (Variables|FormationLocations|GetHit%20Result%20Impact%20Point) (Variables|Default|GetSelectedTroops) 3e+02))
          (Variables|FormationLocations|SetFormationLocations _returnvalue_2))))))

(event Input|KeyboardEvents|C
  (params (Key :type Key%20Structure :default "None")))

(event Input|KeyboardEvents|P
  (params (Key :type Key%20Structure :default "None"))
  (:Pressed
    (CallFunction|SpawnEnemyWave "/Game/Actors/Combat/NewAI/BP_EnemyTroop.BP_EnemyTroop_C")))

(fn ConstructionScript)

(fn SpawnTroop
  (params (spawn%20location :type Vector) (Troom%20Type :type SoldierTypes%20Enum :default "NewEnumerator0") (TroopClass :type BP%20Base%20Troop%20Class%20Reference))
  (bind _returnvalue (Game|SpawnActorfromClass TroopClass (Math|Conversions|ToTransform(Vector) spawn%20location) "AlwaysSpawn" "MultiplyWithRoot" 0 Troom%20Type "NewEnumerator2" false "0.000000,0.000000,0.000000" 0))
  (return _returnvalue))