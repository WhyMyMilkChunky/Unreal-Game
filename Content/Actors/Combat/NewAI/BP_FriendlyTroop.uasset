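; Friendly troop actor for a selectable, command-driven combat unit with health, a selection decal and an overhead action icon.
; Each tick it shows the decal while selected, turns the icon toward the player camera and sets its material and scale from the current Move, Attack Move or Idle command.
; Damage reduces health; because the death check precedes subtraction, a later hit removes it from the troop controller's lists and destroys it.
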(event Custom|Set%20Is%20Selceted
  (params (is%20selected :type Boolean))
  (Variables|Default|SetisSelected is%20selected))

(event EventBeginPlay
  (|CallParentFunction))

(event Collision|EventActorBeginOverlap
  (params (OtherActor :type Actor%20Object%20Reference))
  (|CallParentFunction OtherActor) ; This node is disabled and will not be called.\nDrag off pins to build functionality.
)

(event EventTick
  (params (DeltaSeconds :type Float%20%28single-precision%29))
  (|CallParentFunction DeltaSeconds)
  (CallFunction|BillBoard (Variables|Default|GetActionIcon))
  ;[1 1 1] selected decal
  (Rendering|SetVisibility (Variables|Default|GetDecal) (Variables|Default|GetisSelected) false)
  (CallFunction|SwitchActionIcon (Variables|Default|GetCurrent%20Command) (Variables|Default|GetActionIcon)))

(event Game|Damage|EventAnyDamage
  (params (Damage :type Float%20%28single-precision%29) (DamageType :type Damage%20Type%20Object%20Reference) (InstigatedBy :type Controller%20Object%20Reference) (DamageCauser :type Actor%20Object%20Reference))
  (bind _self self)
  (bind _troopcontroler (Variables|Default|GetTroopcontroler))
  (if (<= (Variables|Default|GetCurrentHealth) 0.0)
    (Utilities|Array|RemoveItem (Variables|/Game/Actors/Combat/NewAI/BP_TroopController.BP_TroopController_C|GetFriendlyTroops _troopcontroler) _self)
    (Utilities|Array|RemoveItem (Variables|/Game/Actors/Combat/NewAI/BP_TroopController.BP_TroopController_C|GetAllTroops _troopcontroler) _self)
    (Utilities|Array|RemoveItem (Variables|/Game/Actors/Combat/NewAI/BP_TroopController.BP_TroopController_C|GetEnemyTroops _troopcontroler) self)
    (Actor|DestroyActor)
    (else
      (Variables|Default|SetCurrentHealth (- (Variables|Default|GetCurrentHealth) Damage)))))

(fn ConstructionScript
  (|CallParentFunction))

(fn BillBoard
  (params (WidgetComponent :type Widget%20Component%20Object%20Reference))
  (bind _returnvalue (Game|GetPlayerController 0))
  (bind _returnvalue_2 (Transformation|GetWorldLocation WidgetComponent))
  (bind _playercameramanager (Variables|/Script/Engine.PlayerController|GetPlayerCameraManager _returnvalue))
  (bind _returnvalue_3 (Camera|GetCameraLocation _playercameramanager))
  (bind _returnvalue_4 (Math|Rotator|FindLookatRotation _returnvalue_2 _returnvalue_3))
  (bind (_roll _pitch _yaw) (Math|Rotator|BreakRotator _returnvalue_4))
  (Transformation|SetWorldRotation WidgetComponent (Math|Rotator|MakeRotator 0.0 _pitch _yaw) false false))

(fn SwitchActionIcon
  (params (Selection :type E_Command%20Enum :default "NewEnumerator0") (Widget%20Component :type Widget%20Component%20Object%20Reference))
  ;[1 1 1] switch troop action icon
  (switch Utilities|FlowControl|Switch|SwitchonE_Command Selection
    (:NewEnumerator0
      (Rendering|Material|SetMaterial Widget%20Component 0 "/Game/Textures/TroopIcons/T_ICON_FOOTSTEPS_Mat.T_ICON_FOOTSTEPS_Mat")
      ;[1 1 1] change scale of image
      (Transformation|SetWorldScale3D Widget%20Component (Variables|Default|GetLarge%20Scale)))
    (:NewEnumerator1
      (Rendering|Material|SetMaterial Widget%20Component 0 "/Game/Textures/TroopIcons/T_ICON_ATTACKING_Mat.T_ICON_ATTACKING_Mat")
      (Transformation|SetWorldScale3D Widget%20Component (Variables|Default|GetLarge%20Scale)))
    (:NewEnumerator2
      (Rendering|Material|SetMaterial Widget%20Component 0 "/Game/Textures/TroopIcons/T_ICON_IDLE_Mat.T_ICON_IDLE_Mat")
      (Transformation|SetWorldScale3D Widget%20Component (Variables|Default|GetSmall%20Scale)))))