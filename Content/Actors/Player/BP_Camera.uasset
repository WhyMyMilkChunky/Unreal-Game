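; Player camera actor that follows the height of the surface beneath it and carries snow and rain weather effects.
; BeginPlay assigns the snow and rain particle assets, and ActivateParticle toggles any system passed to it.
; Each Tick, AdjustCameraHeight traces vertically through the actor and eases it toward the impact point with a swept move.
; The older distance-based height logic remains disconnected, and the leaves system is unused here.
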(event EventBeginPlay
  (Class|NiagaraComponent|SetAsset (Variables|Default|GetFXS_Snow_System) "/Game/Particles/FXS_Snow_System.FXS_Snow_System" true)
  (Class|NiagaraComponent|SetAsset (Variables|Default|GetFXS_Rain_System) "/Game/Particles/FXS_Rain_System.FXS_Rain_System" true))

(event Collision|EventActorBeginOverlap
  (params (OtherActor :type Actor%20Object%20Reference)))

(event EventTick
  (params (DeltaSeconds :type Float%20%28single-precision%29))
  (CallFunction|AdjustCameraHeight DeltaSeconds))

(fn ConstructionScript)

(fn AdjustCameraHeight
  (params (Delta%20Time :type Float%20%28double-precision%29))
  (bind _returnvalue (Transformation|GetActorLocation))
  (LocalVariables|SetDeltaTime Delta%20Time)
  (bind (_outhit _returnvalue_2) (Collision|LineTraceByChannel (+ _returnvalue "0.000000,0.000000,5000.000000") (- _returnvalue "0.000000,0.000000,10000.000000") "TraceTypeQuery5" true 0 "None" true "(R=1.000000,G=0.000000,B=0.000000,A=1.000000)" "(R=0.000000,G=1.000000,B=0.000000,A=1.000000)" 0.0))
  (if _returnvalue_2
    (Transformation|SetActorLocation (Math|Interpolation|VInterpTo (Transformation|GetActorLocation) (.ImpactPoint (Collision|BreakHitResult _outhit)) (LocalVariables|GetDeltaTime) 2.0) true false)
    (return)))

(fn ActivateParticle
  (params (Active :type Boolean) (Particle%20System :type Niagara%20Component%20Object%20Reference))
  (Components|Activation|SetActive Particle%20System Active false))